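; BP_Machinary is an interactable machine that ends the game when the player uses it while holding the machinery key.
; On BeginPlay it binds a handler to its Use event, which checks HasMachinaryKey on PlayerControllerMetus.
; With the key, it consumes the key, shows End_game_screen, disables character input, shows the cursor and unbinds Use.
; ISetPrompt sets the controller's WidgetSelect prompt according to key possession.
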(event `self.ReceiveBeginPlay`
  (add `self.Use` (delegate `Use_machinery_key`)))

(event `Use_machinery_key`
  (bind _asplayer_controller_metus (cast `/Game/Custom/Blueprints/Character/PlayerControllerMetus` (`GameplayStatics.GetPlayerController` 0)))
  (if (`/Game/Custom/Blueprints/Character/PlayerControllerMetus.Has_Machinary_key` _asplayer_controller_metus)
    (set `/Game/Custom/Blueprints/Character/PlayerControllerMetus.Has_Machinary_key` false _asplayer_controller_metus)
    (bind _returnvalue (`|CreateWidget` "/Game/Custom/Widget/New_UI/End_game_screen.End_game_screen_C" _asplayer_controller_metus))
    (`UserWidget.AddToViewport` _returnvalue 0)
    (`self.DisableInput` (cast `/Game/Custom/Blueprints/Character/FirstPersonCharacter_2` (`GameplayStatics.GetPlayerCharacter` 0) :!pure true) _asplayer_controller_metus)
    (clear `self.Use`)
    (set `PlayerController.bShowMouseCursor` true _asplayer_controller_metus)))

(event `/Game/Custom/Blueprints/Interfaces/IInteractible.ISetPrompt`
  (bind _asplayer_controller_metus (cast `/Game/Custom/Blueprints/Character/PlayerControllerMetus` (`GameplayStatics.GetPlayerController` 0)))
  (if (`/Game/Custom/Blueprints/Character/PlayerControllerMetus.Has_Machinary_key` _asplayer_controller_metus)
    (set `/Game/Custom/Blueprints/Character/PlayerControllerMetus.Widget_Select` "NewEnumerator13" _asplayer_controller_metus)
    (else
      (set `/Game/Custom/Blueprints/Character/PlayerControllerMetus.Widget_Select` "NewEnumerator14" _asplayer_controller_metus))))

(fn `UserConstructionScript`
  (`parent.UserConstructionScript`))