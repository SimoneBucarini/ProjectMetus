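; Blueprint function collection whose SanityCheck makes a random true/false roll weighted by the player's sanity tier.
; It reads the FullSanity, MediumSanity and LowSanity flags on player 0's PlayerControllerMetus, in that order, and rolls against the caller-supplied High, Medium or Low weight.
; It returns false when no tier flag is set.
; NewFunction_0 is an empty stub.
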(fn `NewFunction_0`)

(fn `SanityCheck`
  (params (High :type "Float (double-precision)" :default 0.25) (Medium :type "Float (double-precision)" :default 0.5) (Low :type "Float (double-precision)" :default 0.75))
  (returns (Result :type Boolean))
  (locals (Res :type Boolean))
  (bind _asplayer_controller_metus (cast `/Game/Custom/Blueprints/Character/PlayerControllerMetus` (`GameplayStatics.GetPlayerController` null) :!pure true))
  (if (`/Game/Custom/Blueprints/Character/PlayerControllerMetus.Full_Sanity` _asplayer_controller_metus)
    (if (`KismetMathLibrary.RandomBoolWithWeight` High)
      (set `local.Res` true :!label _label)
      (else
        (set `local.Res` false :!label _label_2)))
    (elif (`/Game/Custom/Blueprints/Character/PlayerControllerMetus.Medium_Sanity` _asplayer_controller_metus)
      (if (`KismetMathLibrary.RandomBoolWithWeight` Medium)
        (goto _label)
        (else
          (goto _label_2)))
      (elif (`/Game/Custom/Blueprints/Character/PlayerControllerMetus.Low_Sanity` _asplayer_controller_metus)
        (if (`KismetMathLibrary.RandomBoolWithWeight` Low)
          (goto _label)
          (else
            (goto _label_2)))
        (else
          (goto _label_2)))))
  (return (`local.Res`)))