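; Building volume that tracks whether the player is indoors and stages haunting events.
; The construction script shapes it from a main box plus auxiliary boxes.
; BeginPlay gathers overlapping lanterns and switches, registers lanterns with PlayerControllerMetus, and hides the Horrific actors.
; Entry starts delayed door closing (if a lockpick is inside), blackouts and Horrific reveals, while exit may later shut a random door if the player holds lockpicks.
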(event `self.ReceiveBeginPlay`
  (bind _asplayer_controller_metus (cast `/Game/Custom/Blueprints/Character/PlayerControllerMetus` (`GameplayStatics.GetPlayerController` 0) :!pure true))
  (`|ExecutionSequence`
    (:`then_0`
      ;[1 1 1] Set overlapping Lanterns (box)
      (for _array_element (`self.GetOverlappingActors` "/Game/Custom/Blueprints/BP_Lantern.BP_Lantern_C")
        (bind _asbp_lantern (cast `/Game/Custom/Blueprints/BP_Lantern` _array_element))
        (set `Actor.Tags` (`|MakeArray`) _asbp_lantern)
        (`KismetArrayLibrary.Array_Add` (`self.Lanterns`) _asbp_lantern)
        (`KismetArrayLibrary.Array_Add` (`/Game/Custom/Blueprints/Character/PlayerControllerMetus.Inside_Lanterns` _asplayer_controller_metus) _asbp_lantern))
      ;[1 1 1] Set outside lanterns
      (bind _outactors (`GameplayStatics.GetAllActorsOfClassWithTag` "/Game/Custom/Blueprints/BP_Lantern.BP_Lantern_C" "Outside"))
      (set `/Game/Custom/Blueprints/Character/PlayerControllerMetus.Outside_Lanterns` _outactors _asplayer_controller_metus))
    (:`then_1`
      (for _array_element_2 (`self.GetOverlappingActors` "/Game/Custom/Blueprints/BP_Switch.BP_Switch_C")
        (bind _asbp_switch (cast `/Game/Custom/Blueprints/BP_Switch` _array_element_2))
        (`KismetArrayLibrary.Array_Add` (`self.Switches`) _asbp_switch)))
    (:`then_2`
      (for _array_element_3 (`self.Horrific`)
        (`self.SetActorHiddenInGame` _array_element_3 true)
        (`self.SetActorEnableCollision` _array_element_3 false)))))

(event `self.ReceiveActorBeginOverlap`
  (params (OtherActor :type "Actor Object Reference"))
  (bind _access_doors (`self.Access_Doors`))
  (if (== OtherActor (`GameplayStatics.GetPlayerCharacter` 0))
    (set `/Game/Custom/Blueprints/Character/PlayerControllerMetus.Is_Outside?` false (cast `/Game/Custom/Blueprints/Character/PlayerControllerMetus` (`GameplayStatics.GetPlayerController` 0) :!pure true))
    (set `self.Player_outside_building` false)
    (`KismetSystemLibrary.PrintString` "Inside" true true (struct :`R` 1.0 :`G` 1.0 :`B` 1.0 :`A` 1.0))
    (`KismetSystemLibrary.RetriggerableDelay` 1.5)
    (for _array_element (`self.GetOverlappingActors` "/Game/Custom/Blueprints/BP_Interactible.BP_Interactible_C")
      (bind (_interactibletype _foodtype _medicinetype _keytype) (break `/Game/Custom/Blueprints/Stuctures/Interactible_ENUM_STRUCT` (`/Game/Custom/Blueprints/BP_Interactible.Static Parameters` (cast `/Game/Custom/Blueprints/BP_Interactible` _array_element :!pure true))))
      (if (== _interactibletype 3)
        (if (== _keytype 0)
          (set `self.Lockpick_in` true))))
    (`|ExecutionSequence`
      (:`then_0`
        ;[1 1 1] Close doors
        (`KismetSystemLibrary.RetriggerableDelay` (`KismetMathLibrary.RandomFloatInRange` 2.0 4.0))
        (if (`self.Lockpick_in`)
          (`/Game/Custom/Blueprints/BP_Door.Entity Close the door` (`|GetArrayItem` _access_doors (`KismetMathLibrary.RandomInteger` (`KismetArrayLibrary.Array_Length` _access_doors))))))
      (:`then_1`
        ;[1 1 1] Turn off lanterns
        (`KismetSystemLibrary.RetriggerableDelay` 10.0)
        (for _array_element_2 (`self.Lanterns`)
          (`/Game/Custom/Blueprints/BP_Lantern.Turn off by entity` _array_element_2)))
      (:`then_2`
        ;[1 1 1] Turn off lights
        (`KismetSystemLibrary.RetriggerableDelay` 5.0)
        (for _array_element_3 (`self.Switches`)
          (`/Game/Custom/Blueprints/BP_Switch.TurnOff` _array_element_3)))
      (:`then_3`
        ;[1 1 1] Horrific spawn
        (`KismetSystemLibrary.Delay` 20.0)
        (for _array_element_4 (`self.Horrific`)
          (`self.SetActorHiddenInGame` _array_element_4 false)
          (`self.SetActorEnableCollision` _array_element_4 true))))))

(event `self.ReceiveActorEndOverlap`
  (params (OtherActor :type "Actor Object Reference"))
  (bind _access_doors (`self.Access_Doors`))
  (bind _asplayer_controller_metus (cast `/Game/Custom/Blueprints/Character/PlayerControllerMetus` (`GameplayStatics.GetPlayerController` 0) :!pure true))
  (bind _output (`|GetArrayItem` _access_doors (`KismetMathLibrary.RandomInteger` (`KismetArrayLibrary.Array_Length` _access_doors))))
  (if (== OtherActor (`GameplayStatics.GetPlayerCharacter` 0))
    (set `/Game/Custom/Blueprints/Character/PlayerControllerMetus.Is_Outside?` true _asplayer_controller_metus)
    (set `self.Player_outside_building` true)
    (`KismetSystemLibrary.PrintString` "Outside" true true (struct :`R` 1.0 :`G` 1.0 :`B` 1.0 :`A` 1.0))
    (`KismetSystemLibrary.RetriggerableDelay` (`KismetMathLibrary.RandomFloatInRange` 10.0 60.0))
    (if (`/Game/Custom/Blueprints/BP_Door.Is_Open` _output)
      (if (> (`/Game/Custom/Blueprints/Character/PlayerControllerMetus.Lockpicks_num` _asplayer_controller_metus) 0)
        (`/Game/Custom/Blueprints/BP_Door.Entity Close the door` _output)))))

(fn `UserConstructionScript`
  (for _array_element (`self.Auxiliary_Boxes`)
    (bind _returnvalue (`AddComponent|NODE_AddBoxComponent-2` :`RelativeTransform` _array_element))
    (`KismetArrayLibrary.Array_Add` (`self.Building_collisions`) _returnvalue))
  (`SceneComponent.K2_SetRelativeTransform` (`self.Box`) (`self.Main box Transform`) false false))