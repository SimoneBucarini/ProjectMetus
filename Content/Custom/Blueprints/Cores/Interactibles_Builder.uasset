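; Manager that spawns and removes BP_Interactible actors in the level, driven by PlayerControllerMetus events.
; On BeginPlay it caches placed interactibles as struct and in-game flag arrays, then respawns flagged ones with indices.
; Respawns target an index or a random absent slot of a given type.
; Destroy removes a random interactible from buildings the player is outside, likelier as sanity drops; Z skips the roll.
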(event `Spown`
  (params (`Interactible type` :type "/Game/Custom/Blueprints/Enums/ENUM_interactible Enum" :default "NewEnumerator0"))
  (bind _object_index (`self.Object_index`))
  (bind _returnvalue (`KismetArrayLibrary.Array_Length` _object_index))
  ;[1 1 1] Respawn
  (`KismetArrayLibrary.Array_Clear` (`self.Object_index`))
  (for (_array_element _array_index) (`self.Object_in_game_Array`)
    (if (not _array_element)
      (bind (_output_interactible_transform_parameter _output_static_interactible_parameters) (break `/Game/Custom/Blueprints/Stuctures/Interactible_STRUCT` (`|GetArrayItem` (`self.Array_Struct_Interactible`) _array_index)))
      (if (== (`.Interactibletype_12_305361F248B58E42E7FA4999AEC63E25` (break `/Game/Custom/Blueprints/Stuctures/Interactible_ENUM_STRUCT` _output_static_interactible_parameters)) `Interactible type`)
        (`KismetArrayLibrary.Array_Add` _object_index _array_index))))
  (if (not (<= _returnvalue 0))
    (bind _output_get (set `self.Random_spawn_index` (`|GetArrayItem` _object_index (`KismetMathLibrary.RandomInteger` _returnvalue))))
    (`self.SpawnInteractible` _output_get)))

(event `GenericSpawn`
  (params (Index :type Integer))
  ;[1 1 1] Respawn
  (if (not (`|GetArrayItem` (`self.Object_in_game_Array`) Index))
    (`self.SpawnInteractible` Index)))

(event `Destroy`
  (bind _interactibles_references_array (`self.Interactibles_References_Array`))
  (bind _returnvalue (`KismetArrayLibrary.Array_Length` _interactibles_references_array))
  (bind _asplayer_controller_metus (cast `/Game/Custom/Blueprints/Character/PlayerControllerMetus` (`GameplayStatics.GetPlayerController` 0) :!pure true))
  ;[1 1 1] Destroy Randomizer
  (if (`/Game/Custom/Blueprints/Character/PlayerControllerMetus.Full_Sanity` _asplayer_controller_metus)
    (if (`KismetMathLibrary.RandomBoolWithWeight` 0.25)
      ;[1 1 1] Destroy
      (`KismetArrayLibrary.Array_Clear` (`self.Interactibles_References_Array`) :!label _label)
      (bind _outactors (`GameplayStatics.GetAllActorsOfClass` "/Game/Custom/Blueprints/Cores/Building_box.Building_box_C"))
      (for _array_element _outactors
        (if (`/Game/Custom/Blueprints/Cores/Building_box.Player_outside_building` _array_element)
          (for _array_element_2 (`self.GetOverlappingActors` _array_element "/Game/Custom/Blueprints/BP_Interactible.BP_Interactible_C")
            (bind _asbp_interactible (cast `/Game/Custom/Blueprints/BP_Interactible` _array_element_2))
            (`KismetArrayLibrary.Array_Add` _interactibles_references_array _asbp_interactible))))
      (if (> _returnvalue 0)
        (bind _output_get (set `self.Random_spawn_index` (`KismetMathLibrary.RandomInteger` _returnvalue)))
        (`self.Generic Destry` (`|GetArrayItem` _interactibles_references_array _output_get))))
    (elif (`/Game/Custom/Blueprints/Character/PlayerControllerMetus.Medium_Sanity` _asplayer_controller_metus)
      (if (`KismetMathLibrary.RandomBoolWithWeight` 0.5)
        (goto _label))
      (elif (`/Game/Custom/Blueprints/Character/PlayerControllerMetus.Low_Sanity` _asplayer_controller_metus)
        (if (`KismetMathLibrary.RandomBoolWithWeight` 0.75)
          (goto _label))))))

(event `Key|Z`
  (params (Key :type "Key Structure"))
  ;[1 1 1] Destroy
  (:`Pressed`
    (goto _label)))

(event `Generic Destry`
  (params (Interactable :type "/Game/Custom/Blueprints/BP_Interactible Object Reference"))
  (bind _index (`/Game/Custom/Blueprints/BP_Interactible.Index` Interactable))
  (bind _object_in_game_array (`self.Object_in_game_Array`))
  ;[1 1 1] Destroy
  (if (`|GetArrayItem` _object_in_game_array _index)
    (`KismetArrayLibrary.Array_Set` _object_in_game_array _index)
    (`self.K2_DestroyActor` Interactable)))

(event `self.ReceiveBeginPlay`
  (bind _asplayer_controller_metus (cast `/Game/Custom/Blueprints/Character/PlayerControllerMetus` (`GameplayStatics.GetPlayerController` 0) :!pure true))
  (add `/Game/Custom/Blueprints/Character/PlayerControllerMetus.Destroy` _asplayer_controller_metus (delegate `Destroy`))
  (add `/Game/Custom/Blueprints/Character/PlayerControllerMetus.Spawn_food_event` _asplayer_controller_metus (delegate `Spown`))
  (add `/Game/Custom/Blueprints/Character/PlayerControllerMetus.SpawnInteractible` _asplayer_controller_metus (delegate `GenericSpawn`))
  (add `/Game/Custom/Blueprints/Character/PlayerControllerMetus.DestryInteractable` _asplayer_controller_metus (delegate `Generic Destry`))
  ;[1 1 1] Begin play spawn
  (`self.EnableInput` (cast `/Game/Custom/Blueprints/Character/PlayerControllerMetus` (`GameplayStatics.GetPlayerController` 0) :!pure true))
  (bind _outactors (`GameplayStatics.GetAllActorsOfClass` "/Game/Custom/Blueprints/BP_Interactible.BP_Interactible_C"))
  (bind _output_get (set `self.Interactibles_References_Array` _outactors))
  (set `self.Iteractible number` (`KismetArrayLibrary.Array_Length` _output_get))
  (for _array_element _output_get
    (bind _spawned (`/Game/Custom/Blueprints/BP_Interactible.Spawned` _array_element))
    (`KismetArrayLibrary.Array_Add` (`self.Object_in_game_Array`) _spawned)
    (bind _output_get_2 (set `self.Struct_Interactible` (make `/Game/Custom/Blueprints/Stuctures/Interactible_STRUCT` (`self.GetTransform` _array_element) (`/Game/Custom/Blueprints/BP_Interactible.Static Parameters` _array_element) (`/Game/Custom/Blueprints/BP_Interactible.Randomizer Enable` _array_element) (`/Game/Custom/Blueprints/BP_Interactible.Randomizer Settings` _array_element) _spawned (`/Game/Custom/Blueprints/BP_Interactible.Break_rate` _array_element))))
    (`KismetArrayLibrary.Array_Add` (`self.Array_Struct_Interactible`) _output_get_2)
    (`self.K2_DestroyActor` _array_element))
  (for (_array_element_2 _array_index) (`self.Array_Struct_Interactible`)
    (if (`|GetArrayItem` (`self.Object_in_game_Array`) _array_index)
      (bind (_interactible_transform_parameter _static_interactible_parameters _randomizerenable _randomizer_settings _in_game _break_rate) (break `/Game/Custom/Blueprints/Stuctures/Interactible_STRUCT` _array_element_2))
      (`|SpawnActorFromClass` "/Game/Custom/Blueprints/BP_Interactible.BP_Interactible_C" _interactible_transform_parameter "Undefined" "OverrideRootScale" null _static_interactible_parameters _randomizerenable _randomizer_settings _break_rate true _array_index null))))

(fn `SpawnInteractible`
  (params (Index :type Integer))
  (bind (_output_interactible_transform_parameter _output_static_interactible_parameters _output_randomizerenable _output_randomizer_settings _output_in_game _output_break_rate) (break `/Game/Custom/Blueprints/Stuctures/Interactible_STRUCT` (`|GetArrayItem` (`self.Array_Struct_Interactible`) Index)))
  (`KismetArrayLibrary.Array_Set` (`self.Object_in_game_Array`) Index true)
  (`|SpawnActorFromClass` "/Game/Custom/Blueprints/BP_Interactible.BP_Interactible_C" _output_interactible_transform_parameter "Undefined" "OverrideRootScale" null _output_static_interactible_parameters _output_randomizerenable _output_randomizer_settings _output_break_rate true Index null))

(fn `UserConstructionScript`)