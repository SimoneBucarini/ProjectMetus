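; Builder that rebuilds every BP_Interactible in the level by capturing, destroying and respawning it.
; It stores each actor's transform, static parameters and randomizer settings in a struct array and tracks an in-game flag per entry.
; Respawned actors get their saved settings back, with location jittered randomly by up to one unit in X and Y.
; The Build_Interactibles event and the BluildInteractibles function hold identical copies of this logic.
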(event `Build_Interactibles`
  (bind _returnvalue (`KismetMathLibrary.RandomFloatInRange` -1.0 1.0))
  (bind _outactors (`GameplayStatics.GetAllActorsOfClass` "/Game/Custom/Blueprints/BP_Interactible.BP_Interactible_C"))
  (bind _output_get (set `self.Interactibles_References_Array` _outactors))
  (set `self.Iteractible number` (`KismetArrayLibrary.Array_Length` _output_get))
  (for _array_element _output_get
    (`KismetArrayLibrary.Array_Add` (`self.Object_in_game_Array`))
    (bind _output_get_2 (set `self.Struct_Interactible` (make `/Game/Custom/Blueprints/Stuctures/Interactible_STRUCT` (`Actor.GetTransform` _array_element) (`/Game/Custom/Blueprints/BP_Interactible.Static Parameters` _array_element) (`/Game/Custom/Blueprints/BP_Interactible.Randomizer Enable` _array_element) (`/Game/Custom/Blueprints/BP_Interactible.Randomizer Settings` _array_element))))
    (`KismetArrayLibrary.Array_Add` (`self.Array_Struct_Interactible`) _output_get_2)
    (`Actor.K2_DestroyActor` _array_element))
  (for (_array_element_2 _array_index) (`self.Array_Struct_Interactible`)
    (`KismetArrayLibrary.Array_Set` (`self.Object_in_game_Array`) _array_index true)
    (bind (_interactible_transform_parameter _static_interactible_parameters _randomizerenable _randomizer_settings) (break `/Game/Custom/Blueprints/Stuctures/Interactible_STRUCT` _array_element_2))
    (bind _returnvalue_2 (`|SpawnActorFromClass` "/Game/Custom/Blueprints/BP_Interactible.BP_Interactible_C" (`KismetMathLibrary.MakeTransform` (`KismetMathLibrary.MakeVector` (+ (.x (.location _interactible_transform_parameter)) _returnvalue) (+ (.y (.location _interactible_transform_parameter)) _returnvalue) (.z (.location _interactible_transform_parameter))) (.rotation _interactible_transform_parameter) (.scale _interactible_transform_parameter)) "Undefined" "OverrideRootScale" null null))
    (set `/Game/Custom/Blueprints/BP_Interactible.Static Parameters` _static_interactible_parameters _returnvalue_2)
    (set `/Game/Custom/Blueprints/BP_Interactible.Randomizer Enable` _randomizerenable _returnvalue_2)
    (set `/Game/Custom/Blueprints/BP_Interactible.Randomizer Settings` _randomizer_settings _returnvalue_2)))

(fn `Bluild Interactibles`
  (bind _returnvalue (`KismetMathLibrary.RandomFloatInRange` -1.0 1.0))
  (bind _outactors (`GameplayStatics.GetAllActorsOfClass` "/Game/Custom/Blueprints/BP_Interactible.BP_Interactible_C"))
  (bind _output_get (set `self.Interactibles_References_Array` _outactors))
  (set `self.Iteractible number` (`KismetArrayLibrary.Array_Length` _output_get))
  (for _array_element _output_get
    (`KismetArrayLibrary.Array_Add` (`self.Object_in_game_Array`))
    (bind _output_get_2 (set `self.Struct_Interactible` (make `/Game/Custom/Blueprints/Stuctures/Interactible_STRUCT` (`Actor.GetTransform` _array_element) (`/Game/Custom/Blueprints/BP_Interactible.Static Parameters` _array_element) (`/Game/Custom/Blueprints/BP_Interactible.Randomizer Enable` _array_element) (`/Game/Custom/Blueprints/BP_Interactible.Randomizer Settings` _array_element))))
    (`KismetArrayLibrary.Array_Add` (`self.Array_Struct_Interactible`) _output_get_2)
    (`Actor.K2_DestroyActor` _array_element))
  (for (_array_element_2 _array_index) (`self.Array_Struct_Interactible`)
    (`KismetArrayLibrary.Array_Set` (`self.Object_in_game_Array`) _array_index true)
    (bind (_interactible_transform_parameter _static_interactible_parameters _randomizerenable _randomizer_settings) (break `/Game/Custom/Blueprints/Stuctures/Interactible_STRUCT` _array_element_2))
    (bind _returnvalue_2 (`|SpawnActorFromClass` "/Game/Custom/Blueprints/BP_Interactible.BP_Interactible_C" (`KismetMathLibrary.MakeTransform` (`KismetMathLibrary.MakeVector` (+ (.x (.location _interactible_transform_parameter)) _returnvalue) (+ (.y (.location _interactible_transform_parameter)) _returnvalue) (.z (.location _interactible_transform_parameter))) (.rotation _interactible_transform_parameter) (.scale _interactible_transform_parameter)) "Undefined" "OverrideRootScale" null null))
    (set `/Game/Custom/Blueprints/BP_Interactible.Static Parameters` _static_interactible_parameters _returnvalue_2)
    (set `/Game/Custom/Blueprints/BP_Interactible.Randomizer Enable` _randomizerenable _returnvalue_2)
    (set `/Game/Custom/Blueprints/BP_Interactible.Randomizer Settings` _randomizer_settings _returnvalue_2)))