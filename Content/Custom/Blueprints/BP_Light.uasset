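; Switchable spot light with looping-style hum and flicker sounds, turned on and off through Spot_light_on and Spot_light_off events.
; BeginPlay randomly marks some lights as flickering or as flickering briefly at switch-on, and spawns both attached sounds.
; A timeline serves as the flicker ticker, randomly dipping intensity for short delays and swapping sound pause states.
; The construction script caches the SpotLight's intensity as the full-brightness level.
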(event `Spot_light_on`
  (set `self.Is_on` true)
  (`AudioComponent.SetPaused` (`self.lightCue`) false)
  (if (stale `self.ReceiveBeginPlay` _output_get)
    (`AudioComponent.SetPaused` (`self.FlickerCue`) false :!label _label)
    ;[1 1 1] Flikering
    (`Timeline|Fliker timeline` :`NewTime` 1.0 :!label _label_2
      (:`Update`
        (if (stale _output_get)
          (`|ExecutionSequence`
            (:`then_0`
              (bind _returnvalue (select `bool` (stale _output_get) :`false` 1.0 :`true` 0.2 :!type "Float (single-precision)"))
              (`LightComponent.SetIntensity` (`self.SpotLight`) (* (`self.Light insensity`) (`KismetMathLibrary.FInterpTo` _returnvalue _returnvalue 0.0 0.1)) :!label _label_3))
            (:`then_1`
              (`KismetSystemLibrary.Delay` (`KismetMathLibrary.RandomFloatInRange` 0.1 0.3))
              (set `self.Flicker` false)))
          (else
            (bind _output_get (set `self.Flicker` (`KismetMathLibrary.RandomBoolWithWeight` 0.01)))
            (`AudioComponent.SetPaused` (`self.FlickerCue`) _output_get)
            (`AudioComponent.SetPaused` (`self.lightCue`) _output_get)
            (goto _label_3))))
      (:`Finished`
        (if (and (`self.Is_on`) (`self.Is_flickering`))
          (goto _label_2 :!via `Reverse`))))
    (else
      (if (stale `self.ReceiveBeginPlay` _output_get_2)
        (`|ExecutionSequence`
          (:`then_0`
            (goto _label))
          (:`then_1`
            (`KismetSystemLibrary.Delay` 0.8)
            (`|ExecutionSequence`
              (:`then_0`
                ;[1 1 1] Turn On
                (`AudioComponent.SetPaused` (`self.FlickerCue`) true)
                (goto _label_2 :!via `Stop`))
              (:`then_1`
                (`KismetSystemLibrary.Delay` 0.2))))))
      (`LightComponent.SetIntensity` (`self.SpotLight`) (`self.Light insensity`)))))

(event `self.ReceiveBeginPlay`
  (bind _returnvalue (`KismetMathLibrary.RandomBoolWithWeight` 0.2))
  (bind _spotlight (`self.SpotLight`))
  (bind _output_get (set `self.Is_flickering` _returnvalue))
  (bind _output_get_2 (set `self.Inital Fliker` _returnvalue))
  (bind _returnvalue_2 (`GameplayStatics.SpawnSoundAttached` "/Game/Custom/Audio/HE_Audio/Elecronic/Flicker_Cue.Flicker_Cue" _spotlight "None" (0.0 0.0 0.0) (struct) "KeepRelativeOffset" true 0.5 1.0 0.0 "/Game/Custom/Audio/HE_Audio/_ATT_Profiles/ATT_PhysicsHit.ATT_PhysicsHit" null false))
  (bind _output_get_3 (set `self.FlickerCue` _returnvalue_2))
  (bind _returnvalue_3 (`GameplayStatics.SpawnSoundAttached` "/Game/Custom/Audio/HE_Audio/Elecronic/Light_Cue.Light_Cue" _spotlight "None" (0.0 0.0 0.0) (struct) "KeepRelativeOffset" true 0.5 1.0 0.0 "/Game/Custom/Audio/HE_Audio/_ATT_Profiles/ATT_PhysicsHit.ATT_PhysicsHit" null false))
  (bind _output_get_4 (set `self.lightCue` _returnvalue_3))
  (if (not (`self.Is_on`))
    (`AudioComponent.SetPaused` _output_get_3 true)
    (`AudioComponent.SetPaused` _output_get_4 true)
    (`LightComponent.SetIntensity` (`self.SpotLight`) 0.0)))

(event `Spot_light_off`
  ;[1 1 1] Turn Off
  (set `self.Is_on` false)
  (`LightComponent.SetIntensity` (`self.SpotLight`) 0.0)
  (`AudioComponent.SetPaused` (`self.FlickerCue`) true)
  (`AudioComponent.SetPaused` (`self.lightCue`) true)
  (goto _label_2 :!via `Stop`))

(fn `UserConstructionScript`
  (set `self.Light insensity` (`LightComponentBase.Intensity` (`self.SpotLight`))))