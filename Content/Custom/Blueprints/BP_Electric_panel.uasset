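; Interactive electric panel that powers its linked Switches while it holds a fuse.
; Using an empty panel spends one fuse from PlayerControllerMetus and energizes the switches; the interaction prompt follows the fuse state.
; Tick checks the player's sanity tier and day count against the panel's sanity flags and Day, then removes the fuse and cuts power through a DoOnce.
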(event `self.ReceiveBeginPlay`
  (add `self.Use` (delegate `Put_fuse`))
  (if (`self.Has_fuse`)
    (for _array_element (`self.Switches`)
      (set `/Game/Custom/Blueprints/BP_Switch.Has_energy` true _array_element))
    (else
      (for _array_element_2 (`self.Switches`)
        (set `/Game/Custom/Blueprints/BP_Switch.Has_energy` false _array_element_2)))))

(event `Put_fuse`
  (if (not (`self.Has_fuse`))
    (bind _asplayer_controller_metus (cast `/Game/Custom/Blueprints/Character/PlayerControllerMetus` (`GameplayStatics.GetPlayerController` 0)))
    (bind _fuses_num (`/Game/Custom/Blueprints/Character/PlayerControllerMetus.Fuses_num` _asplayer_controller_metus))
    (if (> _fuses_num 0)
      (set `self.Has_fuse` true)
      (set `/Game/Custom/Blueprints/Character/PlayerControllerMetus.Fuses_num` (- _fuses_num 1) _asplayer_controller_metus)
      (for _array_element (`self.Switches`)
        (set `/Game/Custom/Blueprints/BP_Switch.Has_energy` true _array_element)))))

(event `/Game/Custom/Blueprints/Interfaces/IInteractible.ISetPrompt`
  (bind _asplayer_controller_metus (cast `/Game/Custom/Blueprints/Character/PlayerControllerMetus` (`GameplayStatics.GetPlayerController` 0)))
  (if (`self.Has_fuse`)
    (set `/Game/Custom/Blueprints/Character/PlayerControllerMetus.Widget_Select` "NewEnumerator0" _asplayer_controller_metus)
    (else
      (set `/Game/Custom/Blueprints/Character/PlayerControllerMetus.Widget_Select` "NewEnumerator9" _asplayer_controller_metus))))

(event `self.ReceiveTick`
  (params (DeltaSeconds :type "Float (single-precision)"))
  (bind _asplayer_controller_metus (cast `/Game/Custom/Blueprints/Character/PlayerControllerMetus` (`GameplayStatics.GetPlayerController` 0) :!pure true))
  ;[1 1 1] Destroy fuse
  (if (`self.High_sanity`)
    (if (`/Game/Custom/Blueprints/Character/PlayerControllerMetus.Full_Sanity` _asplayer_controller_metus)
      (if (== (`self.Day`) (`/Game/Custom/Blueprints/Character/PlayerControllerMetus.Days` _asplayer_controller_metus)) :!label _label
        (if (`self.Has_fuse`)
          (`/Engine/EditorBlueprintResources/StandardMacros.DoOnce` false
            (:`Completed`
              (set `self.Has_fuse` false)
              (for _array_element (`self.Switches`)
                (set `/Game/Custom/Blueprints/BP_Switch.Has_energy` false _array_element)))))))
    (elif (`self.Medium_sanity`)
      (if (`/Game/Custom/Blueprints/Character/PlayerControllerMetus.Medium_Sanity` _asplayer_controller_metus)
        (goto _label))
      (elif (`self.Low_sanity`)
        (if (`/Game/Custom/Blueprints/Character/PlayerControllerMetus.Low_Sanity` _asplayer_controller_metus)
          (goto _label))))))

(fn `UserConstructionScript`)