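; Food component for an interactable pickup that the player can eat on the spot or store in their single food slot.
; On BeginPlay it binds the owning interactable's Use and Interact events to eating and storing.
; Eating adds capped Hunger and copies poison settings to PlayerControllerMetus; storing copies food type and icons, or briefly warns if already carrying food.
; Either successful action destroys the pickup, and ISetPrompt sets the controller's prompt widget.
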(event `self.ReceiveBeginPlay`
  (bind _bpinter (`self.bpInter`))
  (add `/Game/Custom/Blueprints/BP_Interactible.Event_Use` _bpinter (delegate `Eat_in_place`))
  (add `/Game/Custom/Blueprints/BP_Interactible.Event_Interact` _bpinter (delegate `Put_in_inventory`)))

(event `Eat_in_place`
  (bind _returnvalue (`GameplayStatics.GetPlayerController` 0))
  (bind _bpinter (`self.bpInter`))
  (bind _asplayer_controller_metus (cast `/Game/Custom/Blueprints/Character/PlayerControllerMetus` _returnvalue))
  (bind _returnvalue_2 (+ (`/Game/Custom/Blueprints/Character/PlayerControllerMetus.Hunger` _asplayer_controller_metus) (`self.Obtain_Hunger`)))
  (if (> _returnvalue_2 1.0)
    (set `/Game/Custom/Blueprints/Character/PlayerControllerMetus.Hunger` 1.0 _asplayer_controller_metus)
    (else
      (set `/Game/Custom/Blueprints/Character/PlayerControllerMetus.Hunger` _returnvalue_2 _asplayer_controller_metus)))
  (set `/Game/Custom/Blueprints/Character/PlayerControllerMetus.Is_poisoned` (`self.Is_poisoned`) _asplayer_controller_metus)
  (set `/Game/Custom/Blueprints/Character/PlayerControllerMetus.Poison_duration` (`self.Poison_duration`) _asplayer_controller_metus)
  (set `/Game/Custom/Blueprints/Character/PlayerControllerMetus.Poison_ratio` (`self.Poison_ratio`) _asplayer_controller_metus)
  (`Actor.DisableInput` _bpinter _returnvalue :!label _label)
  (`Actor.K2_DestroyActor` _bpinter))

(event `Put_in_inventory`
  (bind _asplayer_controller_metus (cast `/Game/Custom/Blueprints/Character/PlayerControllerMetus` (`GameplayStatics.GetPlayerController` 0)))
  (if (`/Game/Custom/Blueprints/Character/PlayerControllerMetus.Has_food` _asplayer_controller_metus)
    (set `/Game/Custom/Blueprints/Character/PlayerControllerMetus.Warning_Widget_Select` "NewEnumerator1" _asplayer_controller_metus)
    (`KismetSystemLibrary.Delay` (`/Game/Custom/Blueprints/Character/PlayerControllerMetus.Warning_delay` _asplayer_controller_metus))
    (set `/Game/Custom/Blueprints/Character/PlayerControllerMetus.Warning_Widget_Select` "NewEnumerator0" _asplayer_controller_metus)
    (else
      (set `/Game/Custom/Blueprints/Character/PlayerControllerMetus.Has_food` true _asplayer_controller_metus)
      (set `/Game/Custom/Blueprints/Character/PlayerControllerMetus.Food_type` (`self.Food`) _asplayer_controller_metus)
      (set `/Game/Custom/Blueprints/Character/PlayerControllerMetus.Food_Icon` (`self.Icon`) _asplayer_controller_metus)
      (set `/Game/Custom/Blueprints/Character/PlayerControllerMetus.Food_N_Icon` (`self.N_Icon`) _asplayer_controller_metus)
      (set `/Game/Custom/Blueprints/Cores/Interact.IsPointed` false (`self.bpInter`))
      (set `/Game/Custom/Blueprints/Character/PlayerControllerMetus.Widget_Select` "NewEnumerator0" _asplayer_controller_metus)
      (goto _label))))

(event `/Game/Custom/Blueprints/Interfaces/IInteractible.ISetPrompt`
  (bind _asplayer_controller_metus (cast `/Game/Custom/Blueprints/Character/PlayerControllerMetus` (`GameplayStatics.GetPlayerController` 0)))
  (set `/Game/Custom/Blueprints/Character/PlayerControllerMetus.Widget_Select` (`self.Prompt_text`) _asplayer_controller_metus))