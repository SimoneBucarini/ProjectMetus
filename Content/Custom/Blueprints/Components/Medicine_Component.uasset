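; Medicine pickup component that lets the player use a medicine on the spot or carry it in a single inventory slot.
; It binds to the interact actor's Use and Interact events: Use adds health to the player controller, Interact stores the medicine's type and icons there.
; If a medicine is already held, it shows a timed warning instead; otherwise either action destroys the actor.
; The prompt event sets the controller's widget selection to its prompt text.
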(event `self.ReceiveBeginPlay`
  (bind _bpinteract (`self.bpInteract`))
  (add `/Game/Custom/Blueprints/BP_Interactible.Event_Use` _bpinteract (delegate `Meds_in_place`))
  (add `/Game/Custom/Blueprints/BP_Interactible.Event_Interact` _bpinteract (delegate `Put_in_invetory`)))

(event `Meds_in_place`
  (bind _returnvalue (`GameplayStatics.GetPlayerController` 0))
  (bind _bpinteract (`self.bpInteract`))
  (bind _asplayer_controller_metus (cast `/Game/Custom/Blueprints/Character/PlayerControllerMetus` _returnvalue))
  (set `/Game/Custom/Blueprints/Character/PlayerControllerMetus.Health` (+ (`/Game/Custom/Blueprints/Character/PlayerControllerMetus.Health` _asplayer_controller_metus) (`self.health obtained`)) _asplayer_controller_metus)
  (`Actor.DisableInput` _bpinteract _returnvalue :!label _label)
  (`Actor.K2_DestroyActor` _bpinteract))

(event `Put_in_invetory`
  (bind _asplayer_controller_metus (cast `/Game/Custom/Blueprints/Character/PlayerControllerMetus` (`GameplayStatics.GetPlayerController` 0)))
  (if (`/Game/Custom/Blueprints/Character/PlayerControllerMetus.Has_medicine` _asplayer_controller_metus)
    (set `/Game/Custom/Blueprints/Character/PlayerControllerMetus.Warning_Widget_Select` "NewEnumerator2" _asplayer_controller_metus)
    (`KismetSystemLibrary.Delay` (`/Game/Custom/Blueprints/Character/PlayerControllerMetus.Warning_delay` _asplayer_controller_metus))
    (set `/Game/Custom/Blueprints/Character/PlayerControllerMetus.Warning_Widget_Select` "NewEnumerator0" _asplayer_controller_metus)
    (else
      (set `/Game/Custom/Blueprints/Character/PlayerControllerMetus.Has_medicine` true _asplayer_controller_metus)
      (set `/Game/Custom/Blueprints/Character/PlayerControllerMetus.Medicine_type` (`self.Medicine`) _asplayer_controller_metus)
      (set `/Game/Custom/Blueprints/Character/PlayerControllerMetus.Medicine_Icon` (`self.Icon`) _asplayer_controller_metus)
      (set `/Game/Custom/Blueprints/Character/PlayerControllerMetus.Medicine_N_Icon` (`self.N_Icon`) _asplayer_controller_metus)
      (set `/Game/Custom/Blueprints/Cores/Interact.IsPointed` false (`self.bpInteract`))
      (set `/Game/Custom/Blueprints/Character/PlayerControllerMetus.Widget_Select` "NewEnumerator0" _asplayer_controller_metus)
      (goto _label))))

(event `/Game/Custom/Blueprints/Interfaces/IInteractible.ISetPrompt`
  (bind _asplayer_controller_metus (cast `/Game/Custom/Blueprints/Character/PlayerControllerMetus` (`GameplayStatics.GetPlayerController` 0)))
  (set `/Game/Custom/Blueprints/Character/PlayerControllerMetus.Widget_Select` (`self.PromptText`) _asplayer_controller_metus))