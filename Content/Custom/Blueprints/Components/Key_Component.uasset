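; Key component that makes an interactible act as a pickup for the player's inventory, with only the Lockpick key type handled.
; It binds to the interactible's interact event and, below the lockpick limit, updates the player controller's count and icon, then destroys the interactible.
; At the limit it briefly switches the controller's warning widget selection.
; A prompt interface event sets the controller's widget selection.
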(event `self.ReceiveBeginPlay`
  (add `/Game/Custom/Blueprints/BP_Interactible.Event_Interact` (`self.BP_Interactible`) (delegate `Put_in_inventory`)))

(event `Put_in_inventory`
  (bind _bp_interactible (`self.BP_Interactible`))
  (bind _asplayer_controller_metus (cast `/Game/Custom/Blueprints/Character/PlayerControllerMetus` (`GameplayStatics.GetPlayerController` 0)))
  (switch `/Game/Custom/Blueprints/Enums/ENUM_Key_Type` (`self.Key_Type`)
    (:`NewEnumerator0`
      (if (< (`/Game/Custom/Blueprints/Character/PlayerControllerMetus.Lockpicks_num` _asplayer_controller_metus) (`self.Max_Lockpicks`))
        (set `/Game/Custom/Blueprints/Character/PlayerControllerMetus.Has_Lockpick` true _asplayer_controller_metus)
        (set `/Game/Custom/Blueprints/Character/PlayerControllerMetus.Lockpicks_num` (+ (`/Game/Custom/Blueprints/Character/PlayerControllerMetus.Lockpicks_num` _asplayer_controller_metus) 1) _asplayer_controller_metus)
        (set `/Game/Custom/Blueprints/Character/PlayerControllerMetus.Lockpick_icon` (`self.Icon`) _asplayer_controller_metus)
        (set `/Game/Custom/Blueprints/Cores/Interact.IsPointed` false _bp_interactible)
        (set `/Game/Custom/Blueprints/Character/PlayerControllerMetus.Widget_Select` "NewEnumerator0" _asplayer_controller_metus)
        (`Actor.DisableInput` _bp_interactible _asplayer_controller_metus)
        (`Actor.K2_DestroyActor` _bp_interactible)
        (else
          (set `/Game/Custom/Blueprints/Character/PlayerControllerMetus.Warning_Widget_Select` "NewEnumerator4" _asplayer_controller_metus)
          (`KismetSystemLibrary.Delay` (`/Game/Custom/Blueprints/Character/PlayerControllerMetus.Warning_delay` _asplayer_controller_metus))
          (set `/Game/Custom/Blueprints/Character/PlayerControllerMetus.Warning_Widget_Select` "NewEnumerator0" _asplayer_controller_metus))))))

(event `/Game/Custom/Blueprints/Interfaces/IInteractible.ISetPrompt`
  (bind _asplayer_controller_metus (cast `/Game/Custom/Blueprints/Character/PlayerControllerMetus` (`GameplayStatics.GetPlayerController` 0)))
  (set `/Game/Custom/Blueprints/Character/PlayerControllerMetus.Widget_Select` (`self.WidgetSelect`) _asplayer_controller_metus))