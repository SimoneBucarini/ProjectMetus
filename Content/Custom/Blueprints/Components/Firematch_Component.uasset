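; Firematch component that makes an interactable actor a match pickup for the player's inventory.
; On BeginPlay it binds to the interact object's event; below the match limit, interaction updates count, flag and icon on PlayerControllerMetus, resets pointing and prompt, then destroys the actor.
; At the limit, it switches the controller's warning widget for a set delay.
; An ISetPrompt event sets the controller's widget selection to the prompt.
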(event `self.ReceiveBeginPlay`
  (add `/Game/Custom/Blueprints/BP_Interactible.Event_Interact` (`self.BpInteract`) (delegate `Put_in_inventory`)))

(event `Put_in_inventory`
  (bind _returnvalue (`GameplayStatics.GetPlayerController` 0))
  (bind _bpinteract (`self.BpInteract`))
  (bind _asplayer_controller_metus (cast `/Game/Custom/Blueprints/Character/PlayerControllerMetus` _returnvalue))
  (if (< (`/Game/Custom/Blueprints/Character/PlayerControllerMetus.Firematch_num` _asplayer_controller_metus) (`self.Max_firematches`))
    (set `/Game/Custom/Blueprints/Character/PlayerControllerMetus.Has_Firematch` true _asplayer_controller_metus)
    (set `/Game/Custom/Blueprints/Character/PlayerControllerMetus.Firematch_num` (+ (`/Game/Custom/Blueprints/Character/PlayerControllerMetus.Firematch_num` _asplayer_controller_metus) 1) _asplayer_controller_metus)
    (set `/Game/Custom/Blueprints/Character/PlayerControllerMetus.Firematch_Icon` (`self.Icon`) _asplayer_controller_metus)
    (set `/Game/Custom/Blueprints/Cores/Interact.IsPointed` false _bpinteract)
    (set `/Game/Custom/Blueprints/Character/PlayerControllerMetus.Widget_Select` "NewEnumerator0" _asplayer_controller_metus)
    (`Actor.DisableInput` _bpinteract _returnvalue)
    (`Actor.K2_DestroyActor` _bpinteract)
    (else
      (set `/Game/Custom/Blueprints/Character/PlayerControllerMetus.Warning_Widget_Select` "NewEnumerator3" _asplayer_controller_metus)
      (`KismetSystemLibrary.Delay` (`/Game/Custom/Blueprints/Character/PlayerControllerMetus.Warning_delay` _asplayer_controller_metus))
      (set `/Game/Custom/Blueprints/Character/PlayerControllerMetus.Warning_Widget_Select` "NewEnumerator0" _asplayer_controller_metus))))

(event `/Game/Custom/Blueprints/Interfaces/IInteractible.ISetPrompt`
  (bind _asplayer_controller_metus (cast `/Game/Custom/Blueprints/Character/PlayerControllerMetus` (`GameplayStatics.GetPlayerController` 0)))
  (set `/Game/Custom/Blueprints/Character/PlayerControllerMetus.Widget_Select` (`self.PromptText`) _asplayer_controller_metus))