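; Fuse pickup component that lets the player collect fuses into an inventory count held on PlayerControllerMetus.
; On BeginPlay it binds to the interact actor's event; an interaction below the fuse limit updates the count, flag and icon, clears the prompt and destroys that actor.
; At the limit it shows a timed warning widget instead.
; An ISetPrompt event sets the controller's prompt widget selection.
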(event `self.ReceiveBeginPlay`
  (add `/Game/Custom/Blueprints/BP_Interactible.Event_Interact` (`self.BP_Interact`) (delegate `Put_in_inventory`)))

(event `Put_in_inventory`
  (bind _bp_interact (`self.BP_Interact`))
  (bind _asplayer_controller_metus (cast `/Game/Custom/Blueprints/Character/PlayerControllerMetus` (`GameplayStatics.GetPlayerController` 0)))
  (if (< (`/Game/Custom/Blueprints/Character/PlayerControllerMetus.Fuses_num` _asplayer_controller_metus) (`self.Max_Fuses`))
    (set `/Game/Custom/Blueprints/Character/PlayerControllerMetus.Has_Fuse` true _asplayer_controller_metus)
    (set `/Game/Custom/Blueprints/Character/PlayerControllerMetus.Fuses_num` (+ (`/Game/Custom/Blueprints/Character/PlayerControllerMetus.Fuses_num` _asplayer_controller_metus) 1) _asplayer_controller_metus)
    (set `/Game/Custom/Blueprints/Character/PlayerControllerMetus.Fuse_icon` (`self.Icon`) _asplayer_controller_metus)
    (set `/Game/Custom/Blueprints/Cores/Interact.IsPointed` false _bp_interact)
    (set `/Game/Custom/Blueprints/Character/PlayerControllerMetus.Widget_Select` "NewEnumerator0" _asplayer_controller_metus)
    (`Actor.DisableInput` _bp_interact _asplayer_controller_metus)
    (`Actor.K2_DestroyActor` _bp_interact)
    (else
      (set `/Game/Custom/Blueprints/Character/PlayerControllerMetus.Warning_Widget_Select` "NewEnumerator6" _asplayer_controller_metus)
      (`KismetSystemLibrary.Delay` (`/Game/Custom/Blueprints/Character/PlayerControllerMetus.Warning_delay` _asplayer_controller_metus))
      (set `/Game/Custom/Blueprints/Character/PlayerControllerMetus.Warning_Widget_Select` "NewEnumerator0" _asplayer_controller_metus))))

(event `/Game/Custom/Blueprints/Interfaces/IInteractible.ISetPrompt`
  (bind _asplayer_controller_metus (cast `/Game/Custom/Blueprints/Character/PlayerControllerMetus` (`GameplayStatics.GetPlayerController` 0)))
  (set `/Game/Custom/Blueprints/Character/PlayerControllerMetus.Widget_Select` (`self.WidgetSelect`) _asplayer_controller_metus))