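; BP_Bed is an interactable bed actor that lets the player rest.
; Its Box overlap events toggle the actor's input and the IsBedNear flag on PlayerControllerMetus for player 0, without checking which actor overlapped.
; Pressing Interact calls Resting on that controller, then disables the bed's input and re-enables it after a fixed delay, with no recheck that the player is still inside the box.
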(event `self.Box.OnComponentBeginOverlap`
  (params (OverlappedComponent :type "PrimitiveComponent Object Reference") (OtherActor :type "Actor Object Reference") (OtherComp :type "PrimitiveComponent Object Reference") (OtherBodyIndex :type Integer) (bFromSweep :type Boolean) (SweepResult :type "HitResult Structure (by ref)"))
  (bind _returnvalue (`GameplayStatics.GetPlayerController` 0))
  (`self.EnableInput` _returnvalue)
  (set `/Game/Custom/Blueprints/Character/PlayerControllerMetus.Is_bed_near?` true (cast `/Game/Custom/Blueprints/Character/PlayerControllerMetus` _returnvalue :!pure true)))

(event `self.Box.OnComponentEndOverlap`
  (params (OverlappedComponent :type "PrimitiveComponent Object Reference") (OtherActor :type "Actor Object Reference") (OtherComp :type "PrimitiveComponent Object Reference") (OtherBodyIndex :type Integer))
  (bind _returnvalue (`GameplayStatics.GetPlayerController` 0))
  (`self.DisableInput` _returnvalue)
  (set `/Game/Custom/Blueprints/Character/PlayerControllerMetus.Is_bed_near?` false (cast `/Game/Custom/Blueprints/Character/PlayerControllerMetus` _returnvalue :!pure true)))

(event `InputAction|Interact`
  (params (Key :type "Key Structure"))
  (bind _returnvalue (`GameplayStatics.GetPlayerController` 0))
  (:`Pressed`
    (`/Game/Custom/Blueprints/Character/PlayerControllerMetus.Resting` (cast `/Game/Custom/Blueprints/Character/PlayerControllerMetus` _returnvalue :!pure true))
    (`self.DisableInput` _returnvalue)
    (`KismetSystemLibrary.Delay` 5.0)
    (`self.EnableInput` _returnvalue)))

(fn `UserConstructionScript`)