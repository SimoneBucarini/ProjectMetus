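; Configurable door actor whose construction script picks door and frame meshes and offsets from DoorType, covering house, white, glass and operating room variants.
; Open, close and FlipFlop toggle events play or reverse one timeline that swings the door on yaw, or slides it on Y for type 10.
; Door collision switches off during movement and returns as query-only.
; Paired DoOnce gates alternate per-type open and close sounds without repeats.
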(event `self.Open Door`
  (bind _door (`self.Door`))
  (bind _door_2 (`self.Door`))
  (bind _door_type (`self.Door_Type`))
  (`|ExecutionSequence` :!label _label
    (:`then_0`
      (`/Engine/EditorBlueprintResources/StandardMacros.DoOnce` false :!label _label_2
        (:`Completed`
          (`GameplayStatics.SpawnSoundAttached` (`BlueprintMapLibrary.Map_Find` (`self.OpenSounds`) _door_type) _door "None" (0.0 0.0 0.0) (struct) "KeepRelativeOffset" false 1.0 1.0 0.0 "/Game/Custom/Audio/HE_Audio/_ATT_Profiles/ATT_PhysicsHit.ATT_PhysicsHit" null)
          (goto _label_5 :!via `Reset`))))
    (:`then_1`
      (`PrimitiveComponent.SetCollisionEnabled` (`self.Door`) "NoCollision")
      (bind (_direction _door_3) (`Timeline|Timeline_1` :!label _label_3)
        (:`Update`
          (if (!= (`self.Door_Type`) 10)
            (`SceneComponent.K2_SetRelativeRotation` _door_2 (`KismetMathLibrary.MakeRotator` 0.0 0.0 _door_3) false false)
            (else
              (`SceneComponent.K2_SetRelativeLocation` _door_2 (`KismetMathLibrary.MakeVector` 0.0 (* -1 _door_3)) false false))))
        (:`Finished`
          (`PrimitiveComponent.SetCollisionEnabled` (`self.Door`) "QueryOnly"))))))

(event `self.Door_Open_Cloose`
  (`/Engine/EditorBlueprintResources/StandardMacros.FlipFlop`
    (:`A`
      (goto _label))
    (:`B`
      (`|ExecutionSequence` :!label _label_4
        (:`then_0`
          (`PrimitiveComponent.SetCollisionEnabled` (`self.Door`) "NoCollision")
          (goto _label_3 :!via `Reverse`))
        (:`then_1`
          (`/Engine/EditorBlueprintResources/StandardMacros.DoOnce` false :!label _label_5
            (:`Completed`
              (`GameplayStatics.SpawnSoundAttached` (`BlueprintMapLibrary.Map_Find` (`self.CloseSounds`) (`self.Door_Type`)) (`self.Door`) "None" (0.0 0.0 0.0) (struct) "KeepRelativeOffset" false 1.0 1.0 0.0 "/Game/Custom/Audio/HE_Audio/_ATT_Profiles/ATT_PhysicsHit.ATT_PhysicsHit" null)
              (goto _label_2 :!via `Reset`))))))))

(event `self.Close Door`
  (goto _label_4))

(fn `UserConstructionScript`
  (locals (House_Door_Location :type "Vector Structure" :default (3e-06 14.736664 8.659424)) (House_Frame_Location :type "Vector Structure" :default (-47.5 12.419222 -4.6e-05)) (Operating_Door_Location :type "Vector Structure" :default (-0.033262 -0.026652 0.0)) (Operating_farame_Location :type "Vector Structure" :default (6.707248 -37.309868 0.0)) (Glass_outdoor :type "Vector Structure" :default (-2.775539 -102.802048 8e-06)) (White_door_location :type "Vector Structure" :default (-1.92207 111.464478 8e-06)) (Stairs_door_location :type "Vector Structure" :default (-2.611859 139.043304 8e-06)))
  (bind _door (`self.Door`))
  (bind _door_2 (`self.Door`))
  (bind _house_door_location (`local.House_Door_Location`))
  (bind _frame (`self.Frame`))
  (bind _frame_2 (`self.Frame`))
  (bind _door_3 (`self.Door`))
  (bind _frame_3 (`self.Frame`))
  (bind _door_4 (`self.Door`))
  (switch `/Game/Custom/Blueprints/Enums/ENUM_Doors` (`self.Door_Type`)
    (:`NewEnumerator0`
      (`StaticMeshComponent.SetStaticMesh` _door_3 "/Game/VillageHousePack_v1/Meshes/DoorMeshes/SM_Door_1.SM_Door_1")
      (`SceneComponent.K2_SetRelativeLocation` _door_3 _house_door_location false false)
      (`ActorComponent.K2_DestroyComponent` (`self.Frame`) :!label _label))
    (:`NewEnumerator1`
      (`StaticMeshComponent.SetStaticMesh` _door "/Game/VillageHousePack_v1/Meshes/DoorMeshes/SM_Door_4.SM_Door_4")
      (`SceneComponent.K2_SetRelativeLocation` _door _house_door_location false false)
      (`StaticMeshComponent.SetStaticMesh` _frame_3 "/Game/VillageHousePack_v1/Meshes/DoorMeshes/SM_Door_Frame_1.SM_Door_Frame_1" :!label _label_2)
      (`SceneComponent.K2_SetRelativeRotation` _frame_3 (struct :`Yaw` 90.0) false false)
      (`SceneComponent.K2_SetRelativeLocation` _frame_3 (`local.House_Frame_Location`) false false))
    (:`NewEnumerator2`
      (`StaticMeshComponent.SetStaticMesh` _door_2 "/Game/VillageHousePack_v1/Meshes/DoorMeshes/SM_Door_2.SM_Door_2")
      (`SceneComponent.K2_SetRelativeLocation` _door_2 _house_door_location false false)
      (goto _label_2))
    (:`NewEnumerator3`
      (`StaticMeshComponent.SetStaticMesh` (`self.Door`) "/Game/Building/Meshes/Building/Door/SM_Doorway_01_Door_01.SM_Doorway_01_Door_01")
      (`StaticMeshComponent.SetStaticMesh` _frame "/Game/Building/Meshes/Building/Door/SM_Doorway_01.SM_Doorway_01")
      (`SceneComponent.K2_SetRelativeLocation` (`self.Door`) (`local.White_door_location`) false false :!label _label_3))
    (:`NewEnumerator4`
      (`StaticMeshComponent.SetStaticMesh` (`self.Door`) "/Game/Building/Meshes/Building/Door/SM_Doorway_01_Door_02.SM_Doorway_01_Door_02")
      (`StaticMeshComponent.SetStaticMesh` _frame "/Game/Building/Meshes/Building/Door/SM_Doorway_01.SM_Doorway_01")
      (goto _label_3))
    (:`NewEnumerator5`
      (`StaticMeshComponent.SetStaticMesh` (`self.Door`) "/Game/Building/Meshes/Building/Door/SM_Stairs_Door.SM_Stairs_Door")
      (`StaticMeshComponent.SetStaticMesh` _frame "/Game/Building/Meshes/Building/Door/SM_Doorway_Stairs.SM_Doorway_Stairs")
      (`SceneComponent.K2_SetRelativeLocation` (`self.Door`) (`local.Stairs_door_location`) false false))
    (:`NewEnumerator6`
      (`StaticMeshComponent.SetStaticMesh` (`self.Door`) "/Game/Building/Meshes/Building/Door/SM_Doorway_02_Door_01.SM_Doorway_02_Door_01")
      (`StaticMeshComponent.SetStaticMesh` _frame "/Game/Building/Meshes/Building/Door/SM_Doorway_02.SM_Doorway_02")
      (`SceneComponent.K2_SetRelativeLocation` (`self.Door`) (0.0 103.0 0.0) false false))
    (:`NewEnumerator7`
      (`StaticMeshComponent.SetStaticMesh` (`self.Door`) "/Game/Building/Meshes/Building/Door/SM_Glass_Partition_Door.SM_Glass_Partition_Door")
      (goto _label))
    (:`NewEnumerator8`
      (`StaticMeshComponent.SetStaticMesh` (`self.Door`) "/Game/Building/Meshes/Building/Door/SM_Entrance_Door_02.SM_Entrance_Door_02")
      (goto _label))
    (:`NewEnumerator10`
      (`StaticMeshComponent.SetStaticMesh` (`self.Door`) "/Game/Building/Meshes/Building/Door/SM_Glass_Partition_Door.SM_Glass_Partition_Door")
      (`SceneComponent.K2_SetRelativeLocation` _frame_2 (`local.Glass_outdoor`) false false)
      (`StaticMeshComponent.SetStaticMesh` _frame_2 "/Game/Building/Meshes/Building/Door/SM_Glass_Partition_01.SM_Glass_Partition_01"))
    (:`NewEnumerator9`
      (`StaticMeshComponent.SetStaticMesh` _door_4 "/Game/Building/Meshes/Building/Door/SM_Operating_Room_Door.SM_Operating_Room_Door")
      (`SceneComponent.K2_SetRelativeLocation` _door_4 (`local.Operating_Door_Location`) false false)
      (`SceneComponent.K2_SetRelativeLocation` _frame_2 (`local.Operating_farame_Location`) false false)
      (`StaticMeshComponent.SetStaticMesh` _frame_2 "/Game/Building/Meshes/Building/Door/SM_Doorway_Operating_Room.SM_Doorway_Operating_Room"))))