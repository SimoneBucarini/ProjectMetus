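; BP_Interactible is a configurable item pickup that becomes a firematch, food, medicine, key, battery or fuse.
; Its construction script takes the type from StaticParameters or randomizes it among enabled categories, then sets the mesh and attaches that type's component with its data.
; Random picks are inline expressions repeated at each use, not cached first.
; Input actions fire Use and Interact dispatchers, and Tick has the component set its prompt while pointed at.
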(event `InputAction|Use in place`
  (params (Key :type "Key Structure"))
  (:`Pressed`
    (`self.Event_Use`)))

(event `InputAction|Interact`
  (params (Key :type "Key Structure"))
  (:`Pressed`
    (`self.Event_Interact`)))

(event `self.ReceiveTick`
  (params (DeltaSeconds :type "Float (single-precision)"))
  (if (`self.IsPointed`)
    (message `/Game/Custom/Blueprints/Interfaces/IInteractible.ISetPrompt` (`self.AttachedComponent`))))

(fn `UserConstructionScript`
  (locals (FOOD_DATA :type "/Game/Custom/Blueprints/Stuctures/FOODS_DATA Structure") (MEDICINES_DATA :type "/Game/Custom/Blueprints/Stuctures/MEDICINES_DATA Structure") (KEYS_DATA :type "/Game/Custom/Blueprints/Stuctures/KEYS_DATA Structure") (STRUCT_BATTERY :type "/Game/Custom/Blueprints/Stuctures/STRUCT_Battery Structure") (FIREMATCH_STRUCT :type "/Game/Custom/Blueprints/Stuctures/STRUCT_Firematch Structure") (FUSE_STRUCT :type "/Game/Custom/Blueprints/Stuctures/STRUCT_Fuse Structure") (`Integers Array` :type "Array of Integer") (`Itegers Key Array` :type "Array of Integer"))
  (bind _randomizer_enable (`self.Randomizer Enable`))
  (bind _integers_array (`local.Integers Array`))
  (bind _itegers_key_array (`local.Itegers Key Array`))
  (bind (_mesh _material _sound _icon _prompt_text) (break `/Game/Custom/Blueprints/Stuctures/STRUCT_Firematch` (`local.FIREMATCH_STRUCT`)))
  (bind (_interactibletype _foodtype _medicinetype _keytype) (break `/Game/Custom/Blueprints/Stuctures/Interactible_ENUM_STRUCT` (`self.Static Parameters`)))
  (bind (_randomizefirematch _randomizefood _randomizemedicine _randomizelockpick _randomizehospitalkey _randomizemachinarykey _randomizebattery _randomizefuse) (break `/Game/Custom/Blueprints/Stuctures/Interactible_Randomizer_Settings_STRUCT` (`self.Randomizer Settings`)))
  (bind (_mesh_2 _material_2 _sound_2 _icon_2 _prompt_text_2) (break `/Game/Custom/Blueprints/Stuctures/STRUCT_Battery` (`local.STRUCT_BATTERY`)))
  (bind (_mesh_3 _material_3 _sound_3 _icon_3 _prompt_text_3) (break `/Game/Custom/Blueprints/Stuctures/STRUCT_Fuse` (`local.FUSE_STRUCT`)))
  (bind _returnvalue (select `bool` (`self.Randomizer Enable`) :`false` _foodtype :`true` (`KismetMathLibrary.Conv_IntToByte` (`KismetMathLibrary.RandomIntegerInRange` 0 (- (enumcount `/Game/Custom/Blueprints/Enums/ENUM_Food_Type`) 1))) :!type "Byte"))
  (bind _returnvalue_2 (select `bool` (`self.Randomizer Enable`) :`false` _medicinetype :`true` (`KismetMathLibrary.Conv_IntToByte` (`KismetMathLibrary.RandomIntegerInRange` 0 (- (enumcount `/Game/Custom/Blueprints/Enums/ENUM_Medicine_Type`) 1))) :!type "Byte"))
  (bind _returnvalue_3 (select `bool` (`self.Randomizer Enable`) :`false` _keytype :`true` (`KismetMathLibrary.Conv_IntToByte` (`|GetArrayItem` _itegers_key_array (`KismetMathLibrary.RandomIntegerInRange` 0 (- (`KismetArrayLibrary.Array_Length` _itegers_key_array) 1)))) :!type "Byte"))
  (bind (_hunger_obtained _poison_ratio _mesh_4 _material_4 _sound_4 _icon_4 _n_icon _prompt_text_4) (break `/Game/Custom/Blueprints/Stuctures/STRUCT_Food` (`|GetArrayItem` (`.Foods_Data_3_4B6153B246894231944104B87E575E65` (break `/Game/Custom/Blueprints/Stuctures/FOODS_DATA` (`local.FOOD_DATA`))) (`KismetMathLibrary.Conv_ByteToInt` _returnvalue))))
  (bind (_health_obtained _mesh_5 _material_5 _sound_5 _icon_5 _n_icon_2 _prompt_text_5) (break `/Game/Custom/Blueprints/Stuctures/STRUCT_Medicine` (`|GetArrayItem` (`.Medicines_Data_3_9D22E482455A2D095A0A53B9D33AA131` (break `/Game/Custom/Blueprints/Stuctures/MEDICINES_DATA` (`local.MEDICINES_DATA`))) (`KismetMathLibrary.Conv_ByteToInt` _returnvalue_2))))
  (bind _returnvalue_4 (select `bool` _randomizer_enable :`false` _interactibletype :`true` (cast `/Game/Custom/Blueprints/Enums/ENUM_interactible` (`KismetMathLibrary.Conv_IntToByte` (`|GetArrayItem` _integers_array (`KismetMathLibrary.RandomIntegerInRange` 0 (- (`KismetArrayLibrary.Array_Length` _integers_array) 1)))))))
  (bind (_key_type _mesh_6 _material_6 _sound_6 _icon_6 _prompt_text_6) (break `/Game/Custom/Blueprints/Stuctures/STRUCT_Key` (`|GetArrayItem` (`.Keys_Data_5_9D22E482455A2D095A0A53B9D33AA131` (break `/Game/Custom/Blueprints/Stuctures/KEYS_DATA` (`local.KEYS_DATA`))) (`KismetMathLibrary.Conv_ByteToInt` _returnvalue_3))))
  (if _randomizer_enable
    (if _randomizefirematch
      (`KismetArrayLibrary.Array_Add` (`local.Integers Array`)))
    (if _randomizefood
      (`KismetArrayLibrary.Array_Add` (`local.Integers Array`) 1))
    (if _randomizemedicine
      (`KismetArrayLibrary.Array_Add` (`local.Integers Array`) 2))
    (if (or _randomizelockpick _randomizehospitalkey _randomizemachinarykey)
      (`KismetArrayLibrary.Array_Add` (`local.Integers Array`) 3)
      (if _randomizelockpick
        (`KismetArrayLibrary.Array_Add` (`local.Itegers Key Array`)))
      (if _randomizehospitalkey
        (`KismetArrayLibrary.Array_Add` (`local.Itegers Key Array`) 1))
      (if _randomizemachinarykey
        (`KismetArrayLibrary.Array_Add` (`local.Itegers Key Array`) 2)))
    (if _randomizebattery
      (`KismetArrayLibrary.Array_Add` (`local.Integers Array`) 4))
    (if _randomizefuse
      (`KismetArrayLibrary.Array_Add` (`local.Integers Array`) 5)))
  (switch `/Game/Custom/Blueprints/Enums/ENUM_interactible` _returnvalue_4
    (:`NewEnumerator0`
      (`StaticMeshComponent.SetStaticMesh` (`self.StaticMesh`) _mesh)
      (bind _returnvalue_5 (`AddComponent|NODE_AddFirematch_Component-0` :`BpInteract` self :`Icon` _icon :`PromptText` _prompt_text))
      (set `self.AttachedComponent` _returnvalue_5))
    (:`NewEnumerator1`
      (`StaticMeshComponent.SetStaticMesh` (`self.StaticMesh`) _mesh_4)
      (bind _returnvalue_6 (`AddComponent|NODE_AddFood_Component-2` :`Food` _returnvalue :`Obtain_Hunger` _hunger_obtained :`Poison_ratio` _poison_ratio :`bpInter` self :`Icon` _icon_4 :`N_Icon` _n_icon :`Prompt_text` _prompt_text_4))
      (set `self.AttachedComponent` _returnvalue_6))
    (:`NewEnumerator2`
      (`StaticMeshComponent.SetStaticMesh` (`self.StaticMesh`) _mesh_5)
      (bind _returnvalue_7 (`AddComponent|NODE_AddMedicine_Component-0` :`Medicine` _returnvalue_2 :`bpInteract` self :`health obtained` _health_obtained :`Icon` _icon_5 :`N_Icon` _n_icon_2 :`PromptText` _prompt_text_5))
      (set `self.AttachedComponent` _returnvalue_7))
    (:`NewEnumerator15`
      (`StaticMeshComponent.SetStaticMesh` (`self.StaticMesh`) _mesh_6)
      (bind _returnvalue_8 (`AddComponent|NODE_AddKey_Component-0` :`Key_Type` _key_type :`BP_Interactible` self :`Icon` _icon_6 :`WidgetSelect` _prompt_text_6))
      (set `self.AttachedComponent` _returnvalue_8))
    (:`NewEnumerator16`
      (`StaticMeshComponent.SetStaticMesh` (`self.StaticMesh`) _mesh_2)
      (bind _returnvalue_9 (`AddComponent|NODE_AddBattery_Component-0` :`BP_Interact` self :`Icon` _icon_2 :`WidgetSelect` _prompt_text_2))
      (set `self.AttachedComponent` _returnvalue_9))
    (:`NewEnumerator17`
      (`StaticMeshComponent.SetStaticMesh` (`self.StaticMesh`) _mesh_3)
      (bind _returnvalue_10 (`AddComponent|NODE_AddFuse_component-0` :`BP_Interact` self :`Icon` _icon_3 :`WidgetSelect` _prompt_text_3))
      (set `self.AttachedComponent` _returnvalue_10)))
  (set `self.Static Parameters` (make `/Game/Custom/Blueprints/Stuctures/Interactible_ENUM_STRUCT` _returnvalue_4 (cast `/Game/Custom/Blueprints/Enums/ENUM_Food_Type` _returnvalue) (cast `/Game/Custom/Blueprints/Enums/ENUM_Medicine_Type` _returnvalue_2) (cast `/Game/Custom/Blueprints/Enums/ENUM_Key_Type` _returnvalue_3))))