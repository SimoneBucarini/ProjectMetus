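; BP_Switch is an interactable switch that turns its attached spot lamps on and off when it has energy.
; BeginPlay binds the toggle to the use event, and a FlipFlop alternates IsOn while looping over AttachedLamps.
; Without energy, it sets a warning widget on PlayerControllerMetus, then switches it again after that controller's warning delay.
; ISetPrompt selects the controller's prompt widget according to IsOn.
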(event `self.ReceiveBeginPlay`
  (add `self.Use` (delegate `Toggle_switch`)))

(event `Toggle_switch`
  (if (`self.Has_energy`)
    (`/Engine/EditorBlueprintResources/StandardMacros.FlipFlop`
      (:`A`
        (set `self.Is_on` true)
        (for _array_element (`self.Attached_lamps`)
          (`/Game/Custom/Blueprints/BP_Light.Spot_light_on` _array_element)))
      (:`B`
        (set `self.Is_on` false)
        (for _array_element_2 (`self.Attached_lamps`)
          (`/Game/Custom/Blueprints/BP_Light.Spot_light_off` _array_element_2))))
    (else
      (bind _asplayer_controller_metus (cast `/Game/Custom/Blueprints/Character/PlayerControllerMetus` (`GameplayStatics.GetPlayerController` 0)))
      (set `/Game/Custom/Blueprints/Character/PlayerControllerMetus.Warning_Widget_Select` "NewEnumerator7" _asplayer_controller_metus)
      (`KismetSystemLibrary.Delay` (`/Game/Custom/Blueprints/Character/PlayerControllerMetus.Warning_delay` _asplayer_controller_metus))
      (set `/Game/Custom/Blueprints/Character/PlayerControllerMetus.Warning_Widget_Select` "NewEnumerator0" _asplayer_controller_metus))))

(event `/Game/Custom/Blueprints/Interfaces/IInteractible.ISetPrompt`
  (bind _asplayer_controller_metus (cast `/Game/Custom/Blueprints/Character/PlayerControllerMetus` (`GameplayStatics.GetPlayerController` 0)))
  (if (`self.Is_on`)
    (set `/Game/Custom/Blueprints/Character/PlayerControllerMetus.Widget_Select` "NewEnumerator8" _asplayer_controller_metus)
    (else
      (set `/Game/Custom/Blueprints/Character/PlayerControllerMetus.Widget_Select` "NewEnumerator7" _asplayer_controller_metus))))

(fn `UserConstructionScript`)