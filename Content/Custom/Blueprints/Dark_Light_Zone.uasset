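; Trigger volume actor that marks a dark or lit zone affecting the player character's sanity.
; When the character's capsule enters the box, a dark zone doubles SanityDecrementation and a light zone sets IsInLight.
; Leaving the box reverses the effect by halving the rate or clearing the flag, with the Dark boolean choosing which behavior applies.
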(event `self.Box.OnComponentBeginOverlap`
  (params (OverlappedComponent :type "PrimitiveComponent Object Reference") (OtherActor :type "Actor Object Reference") (OtherComp :type "PrimitiveComponent Object Reference") (OtherBodyIndex :type Integer) (bFromSweep :type Boolean) (SweepResult :type "HitResult Structure (by ref)"))
  (bind _character (`self.Character`))
  (if (== (`Character.CapsuleComponent` _character) OtherComp)
    (if (`self.Dark`)
      (set `/Game/Custom/Blueprints/Personaggio.Sanity_decrementation` (* 2 (`/Game/Custom/Blueprints/Personaggio.Sanity_decrementation` _character)) _character)
      (else
        (set `/Game/Custom/Blueprints/Personaggio.Is_in_light?` true _character)))))

(event `self.Box.OnComponentEndOverlap`
  (params (OverlappedComponent :type "PrimitiveComponent Object Reference") (OtherActor :type "Actor Object Reference") (OtherComp :type "PrimitiveComponent Object Reference") (OtherBodyIndex :type Integer))
  (bind _character (`self.Character`))
  (if (== OtherComp (`Character.CapsuleComponent` _character))
    (if (`self.Dark`)
      (set `/Game/Custom/Blueprints/Personaggio.Sanity_decrementation` (/ (`/Game/Custom/Blueprints/Personaggio.Sanity_decrementation` _character) 2.0) _character)
      (else
        (set `/Game/Custom/Blueprints/Personaggio.Is_in_light?` false _character)))))

(fn `UserConstructionScript`)