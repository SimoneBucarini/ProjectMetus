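; Lockable hospital double gate that the player unlocks with a key, then toggles open and closed via the Interact input.
; Interacting while locked consumes the player controller's hospital key, or briefly shows a warning widget without one.
; Once unlocked, a DoOnce-guarded FlipFlop plays or reverses a timeline, adding direction-swapped local X offsets to both leaves.
; ISetPrompt sets the controller's prompt widget from the FlipFlop state.
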(event `InputAction|Interact`
  (params (Key :type "Key Structure"))
  (:`Pressed`
    (if (`self.IsLocked`)
      (bind _asplayer_controller_metus (cast `/Game/Custom/Blueprints/Character/PlayerControllerMetus` (`GameplayStatics.GetPlayerController` 0)))
      (if (`/Game/Custom/Blueprints/Character/PlayerControllerMetus.Has_Hospital_key` _asplayer_controller_metus)
        (set `self.IsLocked` false)
        (set `/Game/Custom/Blueprints/Character/PlayerControllerMetus.Has_Hospital_key` false _asplayer_controller_metus)
        (else
          (set `/Game/Custom/Blueprints/Character/PlayerControllerMetus.Warning_Widget_Select` "NewEnumerator12" _asplayer_controller_metus)
          (`KismetSystemLibrary.Delay` (`/Game/Custom/Blueprints/Character/PlayerControllerMetus.Warning_delay` _asplayer_controller_metus))
          (set `/Game/Custom/Blueprints/Character/PlayerControllerMetus.Warning_Widget_Select` "NewEnumerator0" _asplayer_controller_metus)))
      (else
        (`/Engine/EditorBlueprintResources/StandardMacros.DoOnce` false :!label _label
          (:`Completed`
            (bind _isa (`/Engine/EditorBlueprintResources/StandardMacros.FlipFlop`)
              (:`A`
                (bind (_direction _right _left) (`Timeline|Open/Close Gate` :!via `PlayFromStart` :!label _label_2)
                  (:`Update`
                    (`SceneComponent.K2_AddLocalOffset` (`self.LeftGate`) (`KismetMathLibrary.MakeVector` (select `ETimelineDirection` _direction :`Forward` _left :`Backward` _right)) false false)
                    (`SceneComponent.K2_AddLocalOffset` (`self.RightGate`) (`KismetMathLibrary.MakeVector` (select `ETimelineDirection` _direction :`Forward` _right :`Backward` _left)) false false))
                  (:`Finished`
                    (goto _label :!via `Reset`))))
              (:`B`
                (goto _label_2 :!via `ReverseFromEnd`)))))))))

(event `/Game/Custom/Blueprints/Interfaces/IInteractible.ISetPrompt`
  (bind _asplayer_controller_metus (cast `/Game/Custom/Blueprints/Character/PlayerControllerMetus` (`GameplayStatics.GetPlayerController` 0)))
  (if (stale `InputAction|Interact` _isa)
    (set `/Game/Custom/Blueprints/Character/PlayerControllerMetus.Widget_Select` "NewEnumerator11" _asplayer_controller_metus)
    (else
      (set `/Game/Custom/Blueprints/Character/PlayerControllerMetus.Widget_Select` "NewEnumerator10" _asplayer_controller_metus))))

(fn `UserConstructionScript`
  (`parent.UserConstructionScript`))