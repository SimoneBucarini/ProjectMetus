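; Text decal actor that displays configurable world text, which can be revealed by the player's sanity and the day count.
; The construction script applies the text and initial visibility, and BeginPlay registers the actor in a slot of PlayerControllerMetus's Decals array.
; Visibility only reveals the text, when Sanity is at or below its threshold and Days has reached its Day.
; Separate events show or hide it directly.
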(event `self.ReceiveBeginPlay`
  (bind _decals (`/Game/Custom/Blueprints/Character/PlayerControllerMetus.Decals` (cast `/Game/Custom/Blueprints/Character/PlayerControllerMetus` (`GameplayStatics.GetPlayerController` 0) :!pure true)))
  (for (_ _array_index) _decals
    (if (== (`|GetArrayItem` _decals _array_index) null)
      (`KismetArrayLibrary.Array_Set` _decals _array_index self)
      (break))))

(event `Text Visible`
  (`SceneComponent.SetVisibility` (`self.TextRender`) true false))

(event `Text Invisible`
  (`SceneComponent.SetVisibility` (`self.TextRender`) false false))

(fn `UserConstructionScript`
  (`TextRenderComponent.K2_SetText` (`self.TextRender`) (`self.Text`))
  (`SceneComponent.SetVisibility` (`self.TextRender`) (`self.Initial Visibility`) false))

(fn `Visibility`
  (bind _asplayer_controller_metus (cast `/Game/Custom/Blueprints/Character/PlayerControllerMetus` (`GameplayStatics.GetPlayerController` 0) :!pure true))
  (if (<= (`/Game/Custom/Blueprints/Character/PlayerControllerMetus.Sanity` _asplayer_controller_metus) (`self.Sanity`))
    (if (>= (`/Game/Custom/Blueprints/Character/PlayerControllerMetus.Days` _asplayer_controller_metus) (`self.Day`))
      (`SceneComponent.SetVisibility` (`self.TextRender`) true false))))