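; BP_Trigger is a configurable scare trigger volume that drives assigned smoke traps, doors, lanterns, fuse panels, lights, decals, horrific props, sounds and interactables.
; Triggered runs flag-gated "OnBegin" actions; ActorEndOverlap runs matching "OnEnd" ones.
; BeginPlay caches interactable indices for respawning through PlayerControllerMetus.
; Begin overlap only starts a Delay with nothing wired after it, Triggered has no caller here, and switch loops are empty.
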(event `self.ReceiveBeginPlay`
  (bind _interactables (`self.Interactables`))
  (if (and (> (`KismetArrayLibrary.Array_Length` _interactables) 0) (or (`self.Spawn Interactables on End`) (`self.Spawn Interactables on Begin`)))
    (for _array_element _interactables
      (`KismetArrayLibrary.Array_Add` (`self.Interactables Index`) (`/Game/Custom/Blueprints/BP_Interactible.Index` _array_element)))))

(event `self.ReceiveActorBeginOverlap`
  (params (OtherActor :type "Actor Object Reference"))
  (`KismetSystemLibrary.Delay` (`self.Begin Overlap Delay`)))

(event `Triggered`
  (bind _smoke_traps (`self.Smoke Traps`))
  (bind _doors (`self.Doors`))
  (bind _switches (`self.Switches`))
  (bind _decals (`self.Decals`))
  (bind _horrific (`self.Horrific`))
  (bind _asplayer_controller_metus (cast `/Game/Custom/Blueprints/Character/PlayerControllerMetus` (`GameplayStatics.GetPlayerController` 0) :!pure true))
  (`|ExecutionSequence`
    (:`then_0`
      (if (`self.Disactive Smoke Trap on Begin`)
        (for _array_element _smoke_traps
          (`/Game/Custom/Blueprints/BP_Smoke_trap.Disactive Smoke` _array_element))))
    (:`then_1`
      (if (`self.Active Smoke Trap on Begin`)
        (for _array_element_2 _smoke_traps
          (`/Game/Custom/Blueprints/BP_Smoke_trap.Active Smoke` _array_element_2))))
    (:`then_2`
      (if (`self.Open the Doors on Begin`)
        (for _array_element_3 _doors
          (`/Game/Custom/Blueprints/BP_Door.Entity Open the door` _array_element_3))))
    (:`then_3`
      (if (`self.Shut the Doors on Begin`)
        (for _array_element_4 _doors
          (`/Game/Custom/Blueprints/BP_Door.Entity Close the door` _array_element_4))))
    (:`then_4`
      (if (`self.Turn On Switches on Begin`)
        (for _ _switches
          _)))
    (:`then_5`
      (if (`self.Turn Off Switch on Begin`)
        (for _ _switches
          _)))
    (:`then_6`
      (if (`self.Turn Off Lantern on Begin`)
        (for _array_element_5 (`self.Lanterns`)
          (`/Game/Custom/Blueprints/BP_Lantern.Turn off by entity` _array_element_5))))
    (:`then_7`
      (if (`self.Break Fuse in the Panel on Begin`)
        (for _array_element_6 (`self.Electric Panels`)
          (`/Game/Custom/Blueprints/BP_Electric_panel.Entity Destroy fuse` _array_element_6))))
    (:`then_8`
      (if (`self.Destry Interactables on Begin `)
        (for _array_element_7 (`self.Interactables`)
          (`/Game/Custom/Blueprints/Character/PlayerControllerMetus.DestryInteractable` _asplayer_controller_metus _array_element_7))))
    (:`then_9`
      (if (`self.Spawn Interactables on Begin`)
        (for _array_element_8 (`self.Interactables Index`)
          (`/Game/Custom/Blueprints/Character/PlayerControllerMetus.SpawnInteractible` _asplayer_controller_metus _array_element_8))))
    (:`then_10`
      (if (`self.Turn Generic Light Off Begin`)
        (for _array_element_9 (`self.Electric Lights`)
          (`/Game/Custom/Blueprints/BP_Light.Spot_light_off` _array_element_9))))
    (:`then_11`
      (if (`self.Spawn Decal on Begin`)
        (for _array_element_10 _decals
          (`/Game/Custom/Blueprints/Text_Decal.Text Visible` _array_element_10))))
    (:`then_12`
      (if (`self.Destry Decal on Begin`)
        (for _array_element_11 _decals
          (`/Game/Custom/Blueprints/Text_Decal.Text Invisible` _array_element_11))))
    (:`then_13`
      (if (`self.Spawn Horrific on Begin`)
        (for _array_element_12 _horrific
          (`/Game/Custom/Blueprints/Horrific.Horrific Visible` _array_element_12))))
    (:`then_14`
      (if (`self.Destry Horrific on Begin`)
        (for _array_element_13 _horrific
          (`/Game/Custom/Blueprints/Horrific.Horrific Invisible` _array_element_13))))
    (:`then_15`
      (if (`self.Sounds Reproduction on Begin`)
        (bind _audio (`/Game/Custom/Blueprints/BP_Sound.Audio` (stale _array_element_14)))
        (if (`KismetSystemLibrary.IsValid` _audio)
          (if (not (`AudioComponent.IsPlaying` _audio))
            (for _array_element_14 (`self.Sounds`) :!label _label
              (`/Game/Custom/Blueprints/BP_Sound.Play` _array_element_14)))
          (else
            (goto _label)))))))

(event `self.ReceiveActorEndOverlap`
  (params (OtherActor :type "Actor Object Reference"))
  (bind _horrific (`self.Horrific`))
  (bind _smoke_traps (`self.Smoke Traps`))
  (bind _doors (`self.Doors`))
  (bind _switches (`self.Switches`))
  (bind _decals (`self.Decals`))
  (bind _asplayer_controller_metus (cast `/Game/Custom/Blueprints/Character/PlayerControllerMetus` (`GameplayStatics.GetPlayerController` 0) :!pure true))
  (`|ExecutionSequence`
    (:`then_0`
      (if (`self.Disactive Smoke Trap on End`)
        (for _array_element _smoke_traps
          (`/Game/Custom/Blueprints/BP_Smoke_trap.Disactive Smoke` _array_element))))
    (:`then_1`
      (if (`self.Active Smoke Trap on End`)
        (for _array_element_2 _smoke_traps
          (`/Game/Custom/Blueprints/BP_Smoke_trap.Active Smoke` _array_element_2))))
    (:`then_2`
      (if (`self.Open the Doors on End`)
        (for _array_element_3 _doors
          (`/Game/Custom/Blueprints/BP_Door.Entity Open the door` _array_element_3))))
    (:`then_3`
      (if (`self.Shut the Doors on End`)
        (for _array_element_4 _doors
          (`/Game/Custom/Blueprints/BP_Door.Entity Close the door` _array_element_4))))
    (:`then_4`
      (if (`self.Turn On Switches on End`)
        (for _ _switches
          _)))
    (:`then_5`
      (if (`self.Turn Off Switches on End`)
        (for _ _switches
          _)))
    (:`then_6`
      (if (`self.Turn Off Lantern on End`)
        (for _array_element_5 (`self.Lanterns`)
          (`/Game/Custom/Blueprints/BP_Lantern.Turn off by entity` _array_element_5))))
    (:`then_7`
      (if (`self.Break Fuse in the Panel on End`)
        (for _array_element_6 (`self.Electric Panels`)
          (`/Game/Custom/Blueprints/BP_Electric_panel.Entity Destroy fuse` _array_element_6))))
    (:`then_8`
      (if (`self.Destry Interactables on End`)
        (for _array_element_7 (`self.Interactables`)
          (`/Game/Custom/Blueprints/Character/PlayerControllerMetus.DestryInteractable` _asplayer_controller_metus _array_element_7))))
    (:`then_9`
      (if (`self.Spawn Interactables on End`)
        (for _array_element_8 (`self.Interactables Index`)
          (`/Game/Custom/Blueprints/Character/PlayerControllerMetus.SpawnInteractible` _asplayer_controller_metus _array_element_8))))
    (:`then_10`
      (if (`self.Turn Generic Light Off End`)
        (for _array_element_9 (`self.Electric Lights`)
          (`/Game/Custom/Blueprints/BP_Light.Spot_light_off` _array_element_9))))
    (:`then_11`
      (if (`self.Spawn Decal on End`)
        (for _array_element_10 _decals
          (`/Game/Custom/Blueprints/Text_Decal.Text Visible` _array_element_10))))
    (:`then_12`
      (if (`self.Destry Decal on End`)
        (for _array_element_11 _decals
          (`/Game/Custom/Blueprints/Text_Decal.Text Invisible` _array_element_11))))
    (:`then_13`
      (if (`self.Spawn Horrific on End`)
        (for _array_element_12 _horrific
          (`/Game/Custom/Blueprints/Horrific.Horrific Visible` _array_element_12))))
    (:`then_14`
      (if (`self.Destry Horrific on End`)
        (for _array_element_13 _horrific
          (`/Game/Custom/Blueprints/Horrific.Horrific Invisible` _array_element_13))))
    (:`then_15`
      (if (`self.Sounds Reproduction on End`)
        (bind _audio (`/Game/Custom/Blueprints/BP_Sound.Audio` (stale _array_element_14)))
        (if (`KismetSystemLibrary.IsValid` _audio)
          (if (not (`AudioComponent.IsPlaying` _audio))
            (for _array_element_14 (`self.Sounds`) :!label _label_2
              (`/Game/Custom/Blueprints/BP_Sound.Play` _array_element_14)))
          (else
            (goto _label_2)))))))

(fn `UserConstructionScript`)