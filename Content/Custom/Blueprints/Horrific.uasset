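; Horror scare actor that starts hidden, with events that toggle its mesh visibility and box query collision.
; When Hit_by_Trace fires with the player's flashlight on, it runs a one-time scare that rotates the player and drains controller Sanity, clamped at zero.
; A shock sound, red camera fade, camera lock and dampened look input hold briefly.
; It then restores control, flashes the Glitch widget with sound, and hides itself.
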(event `Horrific Visible`
  (`SceneComponent.SetVisibility` (`self.StaticMesh`) true false)
  (`PrimitiveComponent.SetCollisionEnabled` (`self.Box`) "QueryOnly"))

(event `Horrific Invisible`
  (`SceneComponent.SetVisibility` (`self.StaticMesh`) false false :!label _label)
  (`PrimitiveComponent.SetCollisionEnabled` (`self.Box`) "NoCollision"))

(event `self.ReceiveBeginPlay`
  (goto _label))

(event `Hit_by_Trace`
  (bind _returnvalue (`GameplayStatics.GetPlayerController` 0))
  (bind _returnvalue_2 (`GameplayStatics.GetPlayerCameraManager` 0))
  (bind _asplayer_controller_metus (cast `/Game/Custom/Blueprints/Character/PlayerControllerMetus` (`GameplayStatics.GetPlayerController` 0) :!pure true))
  (bind _sanity (`/Game/Custom/Blueprints/Character/PlayerControllerMetus.Sanity` _asplayer_controller_metus))
  (bind _asfirst_person_character_2 (cast `/Game/Custom/Blueprints/Character/FirstPersonCharacter_2` (`GameplayStatics.GetPlayerCharacter` 0)))
  (if (`/Game/Custom/Blueprints/Character/FirstPersonCharacter_2.Flashlight_IsOn` _asfirst_person_character_2)
    (`/Engine/EditorBlueprintResources/StandardMacros.DoOnce` false
      (:`Completed`
        (`self.K2_SetActorRelativeRotation` _asfirst_person_character_2 (`KismetMathLibrary.RInterpTo` (`self.K2_GetActorRotation`) (`KismetMathLibrary.FindLookAtRotation` (`self.K2_GetActorLocation`) (`self.K2_GetActorLocation` _asfirst_person_character_2)) 0.0 1000.0) false false)
        (set `/Game/Custom/Blueprints/Character/PlayerControllerMetus.Sanity` (- _sanity 0.3) _asplayer_controller_metus)
        (if (< _sanity 0.0)
          (set `/Game/Custom/Blueprints/Character/PlayerControllerMetus.Sanity` 0.0 _asplayer_controller_metus))
        (`GameplayStatics.PlaySound2D` "/Game/Custom/Audio/Shock_Horrific_Placeholder1.Shock_Horrific_Placeholder1" 1.0 1.0 0.0 null null)
        (bind _asfirst_person_character_2_2 (cast `/Game/Custom/Blueprints/Character/FirstPersonCharacter_2` (`GameplayStatics.GetPlayerCharacter` 0)))
        (set `/Game/Custom/Blueprints/Character/FirstPersonCharacter_2.Camera_Lock` true _asfirst_person_character_2_2)
        (`PlayerCameraManager.StartCameraFade` _returnvalue_2 0.0 0.5 0.5 (struct :`R` 0.822917 :`B` 0.070265 :`A` 1.0) false true)
        (set `PlayerController.InputYawScale` 0.2 _returnvalue)
        (set `PlayerController.InputRollScale` 0.2 _returnvalue)
        (set `PlayerController.InputPitchScale` -0.2 _returnvalue)
        (`KismetSystemLibrary.Delay` 2.0)
        (`PlayerCameraManager.StartCameraFade` _returnvalue_2 0.5 0.0 0.5 (struct :`R` 0.822917 :`B` 0.070265 :`A` 1.0) false false)
        (set `/Game/Custom/Blueprints/Character/FirstPersonCharacter_2.Camera_Lock` false _asfirst_person_character_2_2)
        (set `PlayerController.InputYawScale` 1.0 _returnvalue)
        (set `PlayerController.InputRollScale` 1.0 _returnvalue)
        (set `PlayerController.InputPitchScale` -1.0 _returnvalue)
        (bind _foundwidgets (`WidgetBlueprintLibrary.GetAllWidgetsOfClass` "/Game/Custom/Widget/New_UI/Glitch.Glitch_C" false))
        (`GameplayStatics.PlaySound2D` "/Game/Custom/Audio/HE_Audio/SFX/Glitch_Cue.Glitch_Cue" 1.0 1.0 0.0 null null)
        (bind _output (`|GetArrayItem` _foundwidgets))
        (`Widget.SetVisibility` _output "Visible")
        (`KismetSystemLibrary.Delay` 0.3)
        (`Widget.SetVisibility` _output "Hidden")
        (`SceneComponent.SetVisibility` (`self.StaticMesh`) false false)
        (`PrimitiveComponent.SetCollisionEnabled` (`self.Box`) "NoCollision")))))

(fn `UserConstructionScript`)