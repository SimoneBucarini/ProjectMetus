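; BP_Gate_Text is a gate sign actor whose text render shows the player's current objective for the hospital key.
; The construction script sets the text to a find-the-doctor prompt.
; Each tick it casts the first player controller to PlayerControllerMetus and switches the text to a hurry message once HasHospitalKey is true.
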(event `self.ReceiveTick`
  (params (DeltaSeconds :type "Float (single-precision)"))
  (if (`/Game/Custom/Blueprints/Character/PlayerControllerMetus.Has_Hospital_key` (cast `/Game/Custom/Blueprints/Character/PlayerControllerMetus` (`GameplayStatics.GetPlayerController` 0) :!pure true))
    (`TextRenderComponent.K2_SetText` (`self.TextRender`) (`self.HURRY`))))

(fn `UserConstructionScript`
  (`TextRenderComponent.K2_SetText` (`self.TextRender`) (`self.FIND THE DOCTOR`)))