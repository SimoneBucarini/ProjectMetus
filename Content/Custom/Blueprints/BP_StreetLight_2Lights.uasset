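; Street light actor that switches on and off through events, driving a point light, bulb material glow and attached sound cues.
; At BeginPlay it randomly picks continuous or startup-only flickering, which a timeline drives with random intensity dips and cue pausing.
; A sphere sized from the light's attenuation radius sets the player controller's IsInStreetLight flag on overlap while lit, clearing it on exit.
; The construction script selects the mesh variant and creates the dynamic bulb material.
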(event `Spot_light_on`
  (set `self.IsOn` true)
  (`AudioComponent.SetPaused` (`self.lightCue`) false)
  (if (stale `self.ReceiveBeginPlay` _output_get) :!label _label
    (`AudioComponent.SetPaused` (`self.FlickerCue`) false :!label _label_2)
    ;[1 1 1] Flikering
    (`Timeline|Timeline_0` :`NewTime` 1.0 :!label _label_3
      (:`Update`
        (if (stale _output_get)
          (`|ExecutionSequence`
            (:`then_0`
              (bind _returnvalue (select `bool` (stale _output_get) :`false` 1.0 :`true` 0.2 :!type "Float (single-precision)"))
              (bind _returnvalue_2 (`KismetMathLibrary.FInterpTo` _returnvalue _returnvalue 0.0 0.1))
              (`LightComponent.SetIntensity` (`self.PointLight`) (* (`self.MaxLightIntensity`) _returnvalue_2) :!label _label_4)
              (`MaterialInstanceDynamic.SetScalarParameterValue` (`self.Bulb`) "Power glow" (* 10.0 _returnvalue_2)))
            (:`then_1`
              (`KismetSystemLibrary.Delay` (`KismetMathLibrary.RandomFloatInRange` 0.1 0.3))
              (set `self.Flicker` false)))
          (else
            (bind _output_get (set `self.Flicker` (`KismetMathLibrary.RandomBoolWithWeight` 0.01)))
            (`AudioComponent.SetPaused` (`self.FlickerCue`) _output_get)
            (`AudioComponent.SetPaused` (`self.lightCue`) _output_get)
            (goto _label_4))))
      (:`Finished`
        (if (and (`self.IsOn`) (`self.IsFlickering`))
          (goto _label_3 :!via `Reverse`))))
    (else
      (if (stale `self.ReceiveBeginPlay` _output_get_2)
        (`|ExecutionSequence`
          (:`then_0`
            (goto _label_2))
          (:`then_1`
            (`KismetSystemLibrary.Delay` 0.8)
            (`|ExecutionSequence`
              (:`then_0`
                ;[1 1 1] Turn On
                (`AudioComponent.SetPaused` (`self.FlickerCue`) true)
                (goto _label_3 :!via `Stop`))
              (:`then_1`
                (`KismetSystemLibrary.Delay` 0.2))))))
      (`LightComponent.SetIntensity` (`self.PointLight`) (`self.MaxLightIntensity`))
      (`MaterialInstanceDynamic.SetScalarParameterValue` (`self.Bulb`) "Power glow" 10.0))))

(event `self.ReceiveBeginPlay`
  (bind _returnvalue (`KismetMathLibrary.RandomBoolWithWeight` 0.1))
  (bind _soundorigin (`self.SoundOrigin`))
  (bind _output_get (set `self.IsFlickering` _returnvalue))
  (bind _output_get_2 (set `self.InitialFlicker` _returnvalue))
  (bind _returnvalue_2 (`GameplayStatics.SpawnSoundAttached` "/Game/Custom/Audio/HE_Audio/Elecronic/Flicker_Cue.Flicker_Cue" _soundorigin "None" (0.0 0.0 0.0) (struct) "KeepRelativeOffset" true 0.5 1.0 0.0 "/Game/Custom/Audio/HE_Audio/_ATT_Profiles/ATT_PhysicsHit.ATT_PhysicsHit" null false))
  (bind _output_get_3 (set `self.FlickerCue` _returnvalue_2))
  (bind _returnvalue_3 (`GameplayStatics.SpawnSoundAttached` "/Game/Custom/Audio/HE_Audio/Elecronic/Light_Cue.Light_Cue" _soundorigin "None" (0.0 0.0 0.0) (struct) "KeepRelativeOffset" true 0.5 1.0 0.0 "/Game/Custom/Audio/HE_Audio/_ATT_Profiles/ATT_PhysicsHit.ATT_PhysicsHit" null false))
  (bind _output_get_4 (set `self.lightCue` _returnvalue_3))
  (if (`self.IsOn`)
    (goto _label)
    (else
      (`AudioComponent.SetPaused` _output_get_3 true)
      (`AudioComponent.SetPaused` _output_get_4 true)
      (`LightComponent.SetIntensity` (`self.PointLight`) 0.0)
      (`MaterialInstanceDynamic.SetScalarParameterValue` (`self.Bulb`) "Power glow" 0.4))))

(event `Spot_light_off`
  ;[1 1 1] Turn Off
  (set `self.IsOn` false)
  (`LightComponent.SetIntensity` (`self.PointLight`) 0.0)
  (`MaterialInstanceDynamic.SetScalarParameterValue` (`self.Bulb`) "Power glow" 0.4)
  (`AudioComponent.SetPaused` (`self.FlickerCue`) true)
  (`AudioComponent.SetPaused` (`self.lightCue`) true)
  (goto _label_3 :!via `Stop`))

(event `self.Sphere.OnComponentBeginOverlap`
  (params (OverlappedComponent :type "PrimitiveComponent Object Reference") (OtherActor :type "Actor Object Reference") (OtherComp :type "PrimitiveComponent Object Reference") (OtherBodyIndex :type Integer) (bFromSweep :type Boolean) (SweepResult :type "HitResult Structure (by ref)"))
  (if (`self.IsOn`)
    (set `/Game/Custom/Blueprints/Character/PlayerControllerMetus.IsInStreetLight` true (cast `/Game/Custom/Blueprints/Character/PlayerControllerMetus` (`GameplayStatics.GetPlayerController` 0) :!pure true))))

(event `self.Sphere.OnComponentEndOverlap`
  (params (OverlappedComponent :type "PrimitiveComponent Object Reference") (OtherActor :type "Actor Object Reference") (OtherComp :type "PrimitiveComponent Object Reference") (OtherBodyIndex :type Integer))
  (set `/Game/Custom/Blueprints/Character/PlayerControllerMetus.IsInStreetLight` false (cast `/Game/Custom/Blueprints/Character/PlayerControllerMetus` (`GameplayStatics.GetPlayerController` 0) :!pure true)))

(fn `UserConstructionScript`
  (`StaticMeshComponent.SetStaticMesh` (`self.SM_Street_Light_02`) (select `bool` (`self.3Lights`) :`false` "/Game/Building/Meshes/Exterior_Elements/SM_Street_Light_02.SM_Street_Light_02" :`true` "/Game/Building/Meshes/Exterior_Elements/SM_Street_Light_01.SM_Street_Light_01" :!type "StaticMesh Object Reference"))
  (bind _returnvalue (`PrimitiveComponent.CreateDynamicMaterialInstance` (`self.SM_Street_Light_02`) 1 null "None"))
  (bind _output_get (set `self.Bulb` _returnvalue))
  (`MaterialInstanceDynamic.SetScalarParameterValue` _output_get "Power glow" 10.0)
  (`SphereComponent.SetSphereRadius` (`self.Sphere`) (* (`LocalLightComponent.AttenuationRadius` (`self.PointLight`)) 0.7) true))