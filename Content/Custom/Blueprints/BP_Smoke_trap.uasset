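; BP_Smoke_trap is a smoke trap actor that flags the player controller as IsInSmoke while the player character overlaps it.
; ActiveSmoke starts the particles and query collision, while a timeline sizes the box from the particle bounds and calls Play on the gas-leak sound every update.
; DisactiveSmoke stops the particles, then after a delay disables collision and silences the sound.
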(event `self.ReceiveBeginPlay`
  (bind _returnvalue (`GameplayStatics.SpawnSoundAttached` "/Game/Custom/Audio/Custom/32_Gas_leaking_escape.32_Gas_leaking_escape" (`self.ParticleSystem`) "None" (0.0 0.0 0.0) (struct) "KeepRelativeOffset" true 1.0 1.0 0.0 "/Game/Custom/Audio/HE_Audio/_ATT_Profiles/ATT_PhysicsHit.ATT_PhysicsHit" null false))
  (bind _output_get (set `self.gas` _returnvalue))
  (`AudioComponent.Stop` _output_get)
  (`ActorComponent.SetActive` (`self.ParticleSystem`) false false))

(event `Active Smoke`
  (`ActorComponent.SetActive` (`self.ParticleSystem`) true false)
  (`PrimitiveComponent.SetCollisionEnabled` (`self.BoxCollision`) "QueryOnly")
  (bind (_direction _newtrack_0) (`Timeline|Timeline_0`)
    (:`Update`
      (`BoxComponent.SetBoxExtent` (`self.BoxCollision`) (* (`.BoxExtent` (`KismetSystemLibrary.GetComponentBounds` (`self.ParticleSystem`))) _newtrack_0) true)
      (`AudioComponent.Play` (`self.gas`) 0.0))))

(event `Disactive Smoke`
  (`ActorComponent.SetActive` (`self.ParticleSystem`) false false)
  (`KismetSystemLibrary.Delay` 10.0)
  (`PrimitiveComponent.SetCollisionEnabled` (`self.BoxCollision`) "NoCollision")
  (`AudioComponent.Stop` (`self.gas`)))

(event `self.ReceiveActorBeginOverlap`
  (params (OtherActor :type "Actor Object Reference"))
  (cast `/Game/Custom/Blueprints/Character/FirstPersonCharacter_2` OtherActor)
  (set `/Game/Custom/Blueprints/Character/PlayerControllerMetus.IsInSmoke` true (cast `/Game/Custom/Blueprints/Character/PlayerControllerMetus` (`GameplayStatics.GetPlayerController` 0) :!pure true)))

(event `self.ReceiveActorEndOverlap`
  (params (OtherActor :type "Actor Object Reference"))
  (cast `/Game/Custom/Blueprints/Character/FirstPersonCharacter_2` OtherActor)
  (set `/Game/Custom/Blueprints/Character/PlayerControllerMetus.IsInSmoke` false (cast `/Game/Custom/Blueprints/Character/PlayerControllerMetus` (`GameplayStatics.GetPlayerController` 0) :!pure true)))

(fn `UserConstructionScript`)