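; Player controller for a survival game, holding health, hunger, sleep, sanity, stamina and a day clock.
; Looping timers advance time and drain stats: sanity falls outside light, while empty hunger or sleep and poison drain health until the death screen appears.
; Food and medicine restore stats, and resting fades the screen, skipping to the next day.
; Debug keys toggle HUD bars, zero health or trigger the sanity- and day-gated light shutoff.
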(event `InputAction|Use Medicine`
  (params (Key :type "Key Structure"))
  (bind _health (`self.Health`))
  (bind _returnvalue (+ (`.Health_Obtained_2_3DC83E9244A40BEE8FC9B1BE36546C86` (break `/Game/Custom/Blueprints/Stuctures/STRUCT_Medicine` (`|GetArrayItem` (`.Medicines_Data_3_9D22E482455A2D095A0A53B9D33AA131` (break `/Game/Custom/Blueprints/Stuctures/MEDICINES_DATA` (`self.Medicine_Data`))) (`KismetMathLibrary.Conv_ByteToInt` (`self.Medicine_type`))))) _health))
  ;[1 1 1] Use Medicine
  (:`Pressed`
    (if (< _health 1.0)
      (if (`self.Has_medicine`)
        (if (> _returnvalue 1.0)
          (set `self.Health` 1.0)
          (else
            (set `self.Health` _returnvalue)))
        (set `self.Has_medicine` false)))))

(event `Key|T`
  (params (Key :type "Key Structure"))
  ;[1 1 1] Turn off lights
  (:`Pressed`
    (`self.E_Turn_off_lights`)))

(event `InputAction|Use Food`
  (params (Key :type "Key Structure"))
  (bind _hunger (`self.Hunger`))
  (bind (_hunger_obtained _poison_ratio _mesh _material _sound _icon _n_icon _prompt_text _poison_duration _is_poisoned) (break `/Game/Custom/Blueprints/Stuctures/STRUCT_Food` (`|GetArrayItem` (`.Foods_Data_3_4B6153B246894231944104B87E575E65` (break `/Game/Custom/Blueprints/Stuctures/FOODS_DATA` (`self.FOOD_DATA`))) (`KismetMathLibrary.Conv_ByteToInt` (`self.Food_type`)))))
  (bind _returnvalue (+ _hunger_obtained _hunger))
  ;[1 1 1] Use Food
  (:`Pressed`
    (if (< _hunger 1.0)
      (if (`self.Has_food`)
        (if (> _returnvalue 1.0)
          (set `self.Hunger` 1.0)
          (else
            (set `self.Hunger` _returnvalue)))
        (set `self.Has_food` false)
        (set `self.Is_poisoned` _is_poisoned)
        (set `self.Poison_duration` _poison_duration)
        (set `self.Poison_ratio` _poison_ratio)))))

(event `Key|B`
  (params (Key :type "Key Structure"))
  (bind _health_bar (`self.health bar`))
  ;[1 1 1] HUD Debug
  (:`Pressed`
    (`|ExecutionSequence`
      (:`then_0`
        (`/Engine/EditorBlueprintResources/StandardMacros.DoOnce` false
          (:`Completed`
            (bind _returnvalue (`|CreateWidget` "/Game/Custom/Widget/New_UI/HUD_HealthBar.HUD_HealthBar_C"))
            (set `self.health bar` _returnvalue)
            (bind _returnvalue_2 (`|CreateWidget` "/Game/Custom/Widget/New_UI/HUD_Sanity.HUD_Sanity_C"))
            (set `self.sanity bar` _returnvalue_2))))
      (:`then_1`
        (`/Engine/EditorBlueprintResources/StandardMacros.FlipFlop`
          (:`A`
            (`UserWidget.AddToViewport` _health_bar 0)
            (`UserWidget.AddToViewport` (`self.sanity bar`) 0))
          (:`B`
            (`Widget.RemoveFromParent` _health_bar)
            (`Widget.RemoveFromParent` (`self.sanity bar`))))))))

(event `Key|K`
  (params (Key :type "Key Structure"))
  (:`Pressed`
    (set `self.Health` 0.0)))

(event `Death`
  (bind _returnvalue (`GameplayStatics.GetPlayerController` 0))
  ;[1 1 1] Death
  (`/Engine/EditorBlueprintResources/StandardMacros.DoOnce` false
    (:`Completed`
      (`self.DisableInput` (`GameplayStatics.GetPlayerPawn` 0) _returnvalue)
      (bind _returnvalue_2 (`|CreateWidget` "/Game/Custom/Widget/New_UI/DeathScreen.DeathScreen_C" _returnvalue))
      (`UserWidget.AddToViewport` _returnvalue_2 0)
      (set `PlayerController.bShowMouseCursor` true _returnvalue)
      (`WidgetBlueprintLibrary.SetInputMode_GameAndUIEx` self _returnvalue_2))))

(event `self.ReceiveBeginPlay`
  (`|ExecutionSequence`
    (:`then_0`
      (set `self.Battery_charge` (`self.Max_battery_charge`))
      (`WidgetBlueprintLibrary.SetInputMode_GameOnly` self)
      (set `self.Sanity_decrementation_saved` (`self.Sanity_Decrementation`))
      (bind _outactors (`GameplayStatics.GetAllActorsOfClass` "/Game/Custom/Blueprints/BP_Switch.BP_Switch_C"))
      (set `self.Light_Switches` _outactors))
    (:`then_1`
      (`KismetSystemLibrary.K2_SetTimer` null "Time" (`self.System Clock`) true)
      (`KismetSystemLibrary.K2_SetTimer` null "Sanity_timer" (`self.Sanity_timer_frequency`) true)
      (`KismetSystemLibrary.K2_SetTimer` null "Hunger_timer" (`self.Hunger_timer_frequency`) true)
      (`KismetSystemLibrary.K2_SetTimer` null "Sleep_Timer" (`self.Sleep__timer_frequency`) true)
      (`KismetSystemLibrary.K2_SetTimer` null "Health Degrowth By Sanity And Hunger" (`self.Health_timer_frequency`) true))))

(event `Resting`
  (bind _returnvalue (`GameplayStatics.GetPlayerCameraManager` 0))
  (bind _returnvalue_2 (`GameplayStatics.GetPlayerPawn` 0))
  ;[1 1 1] Resting
  (if (`self.is_bed_near?`)
    (`self.DisableInput` _returnvalue_2 (`GameplayStatics.GetPlayerController` 0))
    (`self.Rest`)
    (set `self.Resting?` true)
    (`PlayerCameraManager.StartCameraFade` :`self` _returnvalue :`ToAlpha` 1.0 :`Duration` 2.5 :`bHoldWhenFinished` true)
    (`KismetSystemLibrary.Delay` 2.5)
    (`PlayerCameraManager.StartCameraFade` :`self` _returnvalue :`FromAlpha` 1.0 :`Duration` 2.5 :`bHoldWhenFinished` true)
    (`KismetSystemLibrary.Delay` 2.5)
    (`self.EnableInput` _returnvalue_2 (`GameplayStatics.GetPlayerController` 0))
    (set `self.Resting?` false)))

(event `Decrease Stamina`
  (bind _output_get (set `self.Stamina` (- (`self.Stamina`) (`self.Sprint_decrementation`))))
  (set `self.Stop_stamina_drain` (<= _output_get 0.0)))

(event `Stamina Incrementation`
  (bind _output_get (set `self.Stamina` (+ (`self.Stamina`) (`self.Sprint_incrementation`))))
  (set `self.Stop_stamina_regen` (>= _output_get 1.0)))

(event `self.ReceiveTick`
  (params (DeltaSeconds :type "Float (single-precision)"))
  (bind _poison_duration (`self.Poison_duration`))
  (if (>= _poison_duration 0.0)
    (set `self.Poison_duration` (- _poison_duration DeltaSeconds))
    (if (< (`self.Poison_duration`) 0.0)
      (set `self.Is_poisoned` false))))

(fn `E_Turn_off_lights`
  (if (and (`self.Full_Sanity`) (>= (`self.Days`) 2))
    (for _array_element (`self.Light_Switches`) :!label _label
      (`/Game/Custom/Blueprints/BP_Switch.TurnOff` _array_element))
    (for _array_element_2 (`self.Inside_Lanterns`)
      (`/Game/Custom/Blueprints/BP_Lantern.Turn off by entity` _array_element_2))
    (for _array_element_3 (`self.Outside_Lanterns`)
      (`/Game/Custom/Blueprints/BP_Lantern.Turn off by entity` _array_element_3))
    (elif (and (`self.Medium_Sanity`) (>= (`self.Days`) 1))
      (goto _label)
      (elif (and (`self.Low_Sanity`) (>= (`self.Days`) 1))
        (goto _label)))))

(fn `Health Degrowth By Sanity And Hunger`
  (if (<= (`self.Health`) 0.0)
    (set `self.Is_health_zero?` false)
    (`self.Death`)
    (else
      (if (`self.Is_hunger_zero?`)
        (set `self.Health` (- (`self.Health`) (`self.Health_decrementation`))))
      (if (`self.Is_sleep_zero?`)
        (set `self.Health` (- (`self.Health`) (`self.Health_decrementation`))))
      (if (`self.Is_poisoned`)
        (set `self.Health` (- (`self.Health`) (`self.Poison_ratio`)))))))

(fn `Hunger_timer`
  (bind _returnvalue (- (`self.Hunger`) (`self.Hunger_decrementation`)))
  (bind _returnvalue_2 (<= _returnvalue 0.0))
  (if _returnvalue_2
    (set `self.Is_hunger_zero?` _returnvalue_2 :!label _label)
    (set `self.Hunger` 0.0)
    (else
      (set `self.Is_hunger_zero?` _returnvalue_2)
      (if (`self.Is_hunger_zero?`)
        (goto _label)
        (else
          (set `self.Hunger` _returnvalue))))))

(fn `Rest`
  (set `self.Seconds` 0)
  (bind _output_get (set `self.Hours` 8))
  (set `self.Days` (+ (`self.Days`) 1))
  (if (< (`self.Sleep`) 0.3)
    (set `self.Sleep` 0.75)
    (else
      (set `self.Sleep` 1.0))))

(fn `Sanity_timer`
  (bind _sanity (`self.Sanity`))
  (bind _returnvalue (- _sanity (`self.Sanity_decrementation`)))
  (bind _returnvalue_2 (<= _returnvalue 1e-05))
  (if (`self.Resting?`)
    _
    (elif (not (`self.Is_in_light?`))
      (if (>= _sanity 1.0)
        (set `self.Sanity` 1.0))
      (if _returnvalue_2
        (set `self.Is_sanity_zero?` _returnvalue_2 :!label _label)
        (elif (`self.Is_sanity_zero?`)
          (goto _label)
          (else
            (bind _output_get (set `self.Sanity` _returnvalue))
            (if (> _output_get 0.75)
              ;[1 1 1] Sanity Rannge Flags Settings
              (set `self.Low_Sanity` false)
              (set `self.Medium_Sanity` false)
              (set `self.Full_Sanity` true)
              (elif (> _output_get 0.3)
                (set `self.Low_Sanity` false)
                (set `self.Medium_Sanity` true)
                (set `self.Full_Sanity` false)
                (else
                  (set `self.Low_Sanity` true)
                  (set `self.Medium_Sanity` false)
                  (set `self.Full_Sanity` false))))))))))

(fn `Sleep_Timer`
  (bind _returnvalue (- (`self.Sleep`) (`self.Sleep_Decrementation`)))
  (bind _returnvalue_2 (<= _returnvalue 0.0))
  (if _returnvalue_2
    (set `self.Is_sleep_zero?` _returnvalue_2 :!label _label)
    (set `self.Sleep` 0.0)
    (else
      (set `self.Is_sleep_zero?` _returnvalue_2)
      (if (`self.Is_sleep_zero?`)
        (goto _label)
        (else
          (set `self.Sleep` _returnvalue))))))

(fn `Time`
  (bind _decals (`self.Decals`))
  (bind _output_get (set `self.Seconds` (+ (`self.Seconds`) 1)))
  (if (>= _output_get 1)
    (set `self.Seconds` 0)
    (bind _output_get_2 (set `self.Minutes` (+ (`self.Minutes`) 1)))
    (if (>= _output_get_2 60)
      (set `self.Minutes` 0)
      (bind _output_get_3 (set `self.Hours` (+ (`self.Hours`) 1)))
      (if (>= _output_get_3 24)
        (set `self.Hours` 0)
        (set `self.Days` (+ (`self.Days`) 1))
        (for (_ _array_index) _decals
          (`/Game/Custom/Blueprints/Text_Decal.Visibility` (`|GetArrayItem` _decals _array_index)))))))

(fn `UserConstructionScript`)