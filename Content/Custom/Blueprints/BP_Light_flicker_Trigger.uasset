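; Trigger actor that, on any overlap, flickers paired spot and point lights one after another, then operates its linked doors.
; Timeline_1 gates each step, while Timeline_0 scales the current pair's original intensities by its curve.
; After the shorter light array is exhausted, it calls open on each door.
; A Delay inside that loop precedes the close call, so doors open together and only the last closes.
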(event `self.ReceiveActorBeginOverlap`
  (params (OtherActor :type "Actor Object Reference"))
  (bind _spots (`self.Spots`))
  (bind _points (`self.Points`))
  (bind _counter (`self.Counter`))
  (bind _returnvalue (`KismetArrayLibrary.Array_Length` _spots))
  (bind _returnvalue_2 (`KismetArrayLibrary.Array_Length` _points))
  (set `self.Counter` 0)
  (`Timeline|Timeline_1` :`NewTime` (`KismetMathLibrary.RandomFloatInRange` 0.0 2.0) :!label _label
    (:`Finished`
      (`|ExecutionSequence`
        (:`then_0`
          (if (< _counter (select `bool` (<= _returnvalue _returnvalue_2) :`false` _returnvalue_2 :`true` _returnvalue))
            (bind _output_get (set `self.Point Tamplete` (`|GetArrayItem` _points (`self.Counter`))))
            (set `self.Point Intensity` (`LightComponentBase.Intensity` (`Light.LightComponent` _output_get)))
            (bind _output_get_2 (set `self.Spot template` (`|GetArrayItem` _spots (`self.Counter`))))
            (set `self.Spot intensity` (`LightComponentBase.Intensity` (`Light.LightComponent` _output_get_2)))
            (bind (_direction _newtrack_0) (`Timeline|Timeline_0` :!via `PlayFromStart`)
              (:`Update`
                (`LightComponent.SetIntensity` (`Light.LightComponent` (`self.Spot template`)) (* _newtrack_0 (`self.Spot intensity`)))
                (`LightComponent.SetIntensity` (`Light.LightComponent` (`self.Point Tamplete`)) (* _newtrack_0 (`self.Point Intensity`))))
              (:`Finished`
                (`/Engine/EditorBlueprintResources/StandardMacros.IncrementInt` _counter
                  (:`  `
                    (goto _label :!via `PlayFromStart`)))))
            (else
              (`|ExecutionSequence`
                (:`then_0`
                  (goto _label :!via `Stop`))
                (:`then_1`
                  (for _array_element (`self.Doors`)
                    (`/Game/Custom/Blueprints/BP_Door.Entity Open the door` _array_element)
                    (`KismetSystemLibrary.Delay` 2.0)
                    (`/Game/Custom/Blueprints/BP_Door.Entity Close the door` _array_element)))))))
        (:`then_1`
          (goto _label :!via `SetNewTime`))))))

(fn `UserConstructionScript`)